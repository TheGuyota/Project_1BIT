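; Blueprint function library of shared shortcuts that return commonly used game objects already cast to their project types.
; It fetches the first player's character as BP_MainCharacter and the current game mode as BP_InGameGameMode.
; It also resolves a component's owning actor as BP_NPC_Master.
; Each function is a single cast that returns the typed reference only when the cast succeeds.
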(fn `GetMyGameMode`
  (returns (MyGameMode :type "/Game/Blueprints/Core/InGameController/BP_InGameGameMode Object Reference"))
  (bind _asbp_in_game_game_mode (cast `/Game/Blueprints/Core/InGameController/BP_InGameGameMode` (`GameplayStatics.GetGameMode` null)))
  (return _asbp_in_game_game_mode))

(fn `GetMyPlayerCharacter`
  (returns (MainCharacter :type "/Game/Characters/MainCharacter/BP_MainCharacter Object Reference"))
  (bind _asbp_main_character (cast `/Game/Characters/MainCharacter/BP_MainCharacter` (`GameplayStatics.GetPlayerCharacter` null)))
  (return _asbp_main_character))

(fn `GetOwnerNPC`
  (params (Component :type "ActorComponent Object Reference"))
  (returns (NPCSelfRef :type "/Game/Blueprints/NPCs/BP_NPC_Master Object Reference"))
  (bind _asbp_npc_master (cast `/Game/Blueprints/NPCs/BP_NPC_Master` (`ActorComponent.GetOwner` Component)))
  (return _asbp_npc_master))