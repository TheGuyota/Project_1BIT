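; Actor component that stores the player's inventory as a map of items to quantities.
; AddToInventory adds to the existing count, reports the item name and quantity to the player character as an objective ID event, then refreshes the inventory container on that character.
; QueryInventory returns the stored quantity for a given item.
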(fn `AddToInventory`
  (params (Item :type Name) (Quantity :type Integer))
  (bind _maincharacter (`/Game/Blueprints/CommonFuntionLibrary.GetMyPlayerCharacter`))
  (`BlueprintMapLibrary.Map_Add` (`self.Content`) Item (+ Quantity (`BlueprintMapLibrary.Map_Find` (`self.Content`) Item)))
  (`/Game/Characters/MainCharacter/BP_MainCharacter.OnObjectiveIDCalled` _maincharacter (`KismetStringLibrary.Conv_NameToString` (`local.Item`)) (`local.Quantity`))
  (`/Game/Characters/MainCharacter/BP_MainCharacter.UpdateInventoryContainer` _maincharacter))

(fn `QueryInventory`
  (params (Item :type Name))
  (returns (Value :type Integer))
  (return (`BlueprintMapLibrary.Map_Find` (`self.Content`) Item)))