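; Dialogue component for the Hobo (Barbone) NPC, who begs the player for spare change and later offers small talk.
; The first tree branches on a "Monetina" in the inventory: handing it over progresses the DaiMonetina objective, removes the coin, updates the side quest and unlocks the second tree.
; The second tree discusses the gas station cashier, adding a monsters question when the "Mostro" global parameter is set.
; Chained AddDialogue calls drive each branch.
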(fn `Dialogue`
  (switch `int` (`self.DialogueTreeIndex`)
    (:`0`
      (if (`.bIsFound` (`/Game/Blueprints/Components/AC_Inventory.QueryInventory` (`/Game/Characters/MainCharacter/BP_MainCharacter.InventoryComponent` (`/Game/Blueprints/CommonFuntionLibrary.GetMyPlayerCharacter`)) "Monetina"))
        (bind (_state _optionindex) (`self.AddDialogue` "Hobo" "Hey! HEY! Little girl! Do you have some spare change?" true (`|MakeArray` "Here, I don't need it." "Nope." :!type "Text")))
        (switch `/Game/Blueprints/Components/Dialogues/E_DialogueState` _state
          (:`NewEnumerator0`
            (switch `int` _optionindex
              (:`0`
                (bind _state_2 (`self.AddDialogue` "Hobo" "HEH! This quarter goes straight to my booze fund..." false (`|MakeArray` "" :!type "Text")))
                (switch `/Game/Blueprints/Components/Dialogues/E_DialogueState` _state_2
                  (:`NewEnumerator0`
                    (`self.ProgressDialogueQuest` "DaiMonetina" 1)
                    (`/Game/Blueprints/Components/AC_Inventory.RemoveFromInventory` (`/Game/Characters/MainCharacter/BP_MainCharacter.InventoryComponent` (`/Game/Blueprints/CommonFuntionLibrary.GetMyPlayerCharacter`)) "Monetina" 1)
                    (`self.CheckAndUpdateSideQuest`)
                    (`self.SetDialogueTreeIndex` 1)
                    (`self.CloseConversation`))))
              (:`1`
                (bind _state_3 (`self.AddDialogue` "Hobo" "Awwww... Don't bother me then..." true (`|MakeArray` "Pff, how rude!" :!type "Text") :!label _label))
                (switch `/Game/Blueprints/Components/Dialogues/E_DialogueState` _state_3
                  (:`NewEnumerator0`
                    (`self.ClearDialogueProgress`)
                    (`self.CloseConversation`)))))))
        (else
          (bind (_state_4 _optionindex_2) (`self.AddDialogue` "Hobo" "Hey! HEY! Little girl! Do you have some spare change?" true (`|MakeArray` "Where do I get some spare change?" "Nope." :!type "Text")))
          (switch `/Game/Blueprints/Components/Dialogues/E_DialogueState` _state_4
            (:`NewEnumerator0`
              (switch `int` _optionindex_2
                (:`0`
                  (bind _state_5 (`self.AddDialogue` "Hobo" "Just BUY something!" true (`|MakeArray` "I'll head to the gas station store." :!type "Text")))
                  (switch `/Game/Blueprints/Components/Dialogues/E_DialogueState` _state_5
                    (:`NewEnumerator0`
                      (`self.ClearDialogueProgress`)
                      (`self.CloseConversation`))))
                (:`1`
                  (goto _label))))))))
    (:`1`
      (bind (_state_6 _optionindex_3) (`self.AddDialogue` "Hobo" "It's you again! Do you have more quarters? No? Alright... What ya want?" true (select `bool` (>= (`.Quantity` (`self.QueryGlobalParameters` "Mostro")) 1) :`false` (`|MakeArray` "Do you know the cashier dude at the gas station?" :!type "Text") :`true` (`|MakeArray` "Do you know the cashier dude at the gas station?" "Mr. Hobo, can you see the monsters?" :!type "Text"))))
      (switch `/Game/Blueprints/Components/Dialogues/E_DialogueState` _state_6
        (:`NewEnumerator0`
          (switch `int` _optionindex_3
            (:`0`
              (bind _state_7 (`self.AddDialogue` "Hobo" "Ah, that boy... He often gives me leftover sandwiches after his shift. He's a good dude, hard to find people like him these days..." false (`|MakeArray` "" :!type "Text")))
              (switch `/Game/Blueprints/Components/Dialogues/E_DialogueState` _state_7
                (:`NewEnumerator0`
                  (`self.ClearDialogueProgress`)
                  (`self.CloseConversation`))))
            (:`1`
              (bind _state_8 (`self.AddDialogue` "Hobo" "Monsters? HAHAHAHA! This town is full of monsters, kid, otherwise I wouldn't be here. Listen to this old dude, I... Agh, nevermind, you'll get it when you grow up..." false (`|MakeArray` "" :!type "Text")))
              (switch `/Game/Blueprints/Components/Dialogues/E_DialogueState` _state_8
                (:`NewEnumerator0`
                  (`self.ClearDialogueProgress`)
                  (`self.CloseConversation`))))))))))