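; Dialogue component for the BaristaBiker NPC, holding an Italian conversation in which the player asks about a lost kitten and is pointed to the minimarket.
; The Dialogue graph switches on DialogueTreeIndex and chains AddDialogue calls, branching on the chosen option.
; Getting the hint advances the tree to a repeat-visit branch that can restate it.
; Other endings clear dialogue progress before closing the conversation.
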(fn `Dialogue`
  (switch `int` (`self.DialogueTreeIndex`)
    (:`0`
      (bind (_state _optionindex) (`self.AddDialogue` "BaristaBiker" "Dimmi ragazzina" true (`|MakeArray` "Hai visto il mio gattino?" "Niente, ciao" :!type "Text")))
      (switch `/Game/Blueprints/Components/Dialogues/E_DialogueState` _state
        (:`NewEnumerator0`
          (switch `int` _optionindex
            (:`0`
              (bind _state_2 (`self.AddDialogue` "BaristaBiker" "Mmmh... In effetti ho visto un gattino che passava di qui, mi sembra andasse verso il  minimarket" false (`|MakeArray` "" :!type "Text")))
              (switch `/Game/Blueprints/Components/Dialogues/E_DialogueState` _state_2
                (:`NewEnumerator0`
                  (`self.SetDialogueTreeIndex` 1)
                  (`self.CloseConversation`))))
            (:`1`
              (`self.ClearDialogueProgress`)
              (`self.CloseConversation`))))))
    (:`1`
      (bind (_state_3 _optionindex_2) (`self.AddDialogue` "BaristaBiker" "Di nuovo qui?  \nTi sei già scordata dove è andato il gatto?" true (`|MakeArray` "...Si..." "Nah, stavo solo passando di qui" :!type "Text")))
      (switch `/Game/Blueprints/Components/Dialogues/E_DialogueState` _state_3
        (:`NewEnumerator0`
          (switch `int` _optionindex_2
            (:`0`
              (bind _state_4 (`self.AddDialogue` "BaristaBiker" "Ho visto un gattino passare di qui e andare verso il minimarket" true (`|MakeArray` "Graaaazie!" :!type "Text")))
              (switch `/Game/Blueprints/Components/Dialogues/E_DialogueState` _state_4
                (:`NewEnumerator0`
                  (bind _state_5 (`self.AddDialogue` "BaristaBiker" "Ora vai dai che devo lavorare." false (`|MakeArray` "" :!type "Text")))
                  (switch `/Game/Blueprints/Components/Dialogues/E_DialogueState` _state_5
                    (:`NewEnumerator0`
                      (`self.ClearDialogueProgress`)
                      (`self.CloseConversation`))))))
            (:`1`
              (`self.ClearDialogueProgress`)
              (`self.CloseConversation`))))))))