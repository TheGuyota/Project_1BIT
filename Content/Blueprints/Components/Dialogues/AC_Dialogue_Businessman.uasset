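; Dialogue component for the Businessman NPC, playing a short Italian line that depends on his story state.
; Dialogue reads the "Businessman" global parameter and picks a despairing or self-encouraging line, each with a single "..." option.
; Pass Through clears dialogue progress and closes the conversation, as does a missing parameter after printing an error.
; Tick prints the parameter value every frame as debug output.
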(event `self.ReceiveTick`
  (params (DeltaSeconds :type "Float (single-precision)"))
  (`KismetSystemLibrary.PrintString` (`KismetTextLibrary.Conv_TextToString` (`|FormatText` "GlobalParameter: \nBusinessman : {value}" (`.Quantity` (`self.QueryGlobalParameters` "Businessman")))) true true (struct :`G` 0.66 :`B` 1.0 :`A` 1.0) 0.0))

(fn `Dialogue`
  (bind (_bisfound _quantity) (`self.QueryGlobalParameters` "Businessman"))
  (if _bisfound
    (switch `int` _quantity
      (:`0`
        (bind _state (`self.AddDialogue` "Businessman" "...Come è possibile.. Come è potuto succedere.. Perché a me... Non è giusto..." true (`|MakeArray` "..." :!type "Text")))
        (switch `/Game/Blueprints/Components/Dialogues/E_DialogueState` _state
          (:`NewEnumerator0`
            (`self.ClearDialogueProgress`)
            (`self.CloseConversation`))))
      (:`1`
        (bind _state_2 (`self.AddDialogue` "Businessman" "Posso farcela... Posso farcela..." true (`|MakeArray` "..." :!type "Text")))
        (switch `/Game/Blueprints/Components/Dialogues/E_DialogueState` _state_2
          (:`NewEnumerator0`
            (`self.ClearDialogueProgress`)
            (`self.CloseConversation`)))))
    (else
      (`KismetSystemLibrary.PrintString` "ERROR")
      (`self.ClearDialogueProgress`)
      (`self.CloseConversation`))))