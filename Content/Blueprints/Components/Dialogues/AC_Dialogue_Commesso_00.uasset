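; Dialogue component for the Commesso (shop clerk), who offers information on the player's missing kitten in exchange for buying milk.
; AddDialogue calls chain into a branching Italian conversation, offering payment only when the inventory holds a Dollaro.
; Paying advances the BuyMilk objective and removes the dollar on the Updated output.
; Finishing the purchase conversation switches DialogueTreeIndex to a short repeat conversation; refusal rewinds progress.
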(fn `Dialogue`
  (switch `int` (`self.DialogueTreeIndex`)
    (:`0`
      (bind _state (`self.AddDialogue` "Commesso" "Hey tu! Ragazzina!" true (`|MakeArray` "Mh.." :!type "Text")))
      (switch `/Game/Blueprints/Components/Dialogues/E_DialogueState` _state
        (:`NewEnumerator0`
          (bind _state_2 (`self.AddDialogue` "Commesso" "Vuoi comprare qualcosa?" true (`|MakeArray` "Per caso hai visto il mio gattino?" :!type "Text")))
          (switch `/Game/Blueprints/Components/Dialogues/E_DialogueState` _state_2
            (:`NewEnumerator0`
              (bind (_state_3 _optionindex) (`self.AddDialogue` "Commesso" "Mmh... Se compri quel cartone di latte ti dico tutto quello che so." true (`|MakeArray` "Quanto costa il latte..." "Mi stai ricattando?" :!type "Text")))
              (switch `/Game/Blueprints/Components/Dialogues/E_DialogueState` _state_3
                (:`NewEnumerator0`
                  (switch `int` _optionindex
                    (:`0`
                      _)
                    (:`1`
                      (bind _state_4 (`self.AddDialogue` "Commesso" "Si." false (`|MakeArray` "" :!type "Text")))
                      (switch `/Game/Blueprints/Components/Dialogues/E_DialogueState` _state_4
                        (:`NewEnumerator0`
                          _))))
                  (bind (_state_5 _optionindex_2) (`self.AddDialogue` "Commesso" "Il latte costa 80c." true (select `bool` (`.bIsFound` (`/Game/Blueprints/Components/AC_Inventory.QueryInventory` (`/Game/Characters/MainCharacter/BP_MainCharacter.InventoryComponent` (`/Game/Blueprints/CommonFuntionLibrary.GetMyPlayerCharacter`)) "Dollaro")) :`false` (`|MakeArray` "Non ho i soldi." :!type "Text") :`true` (`|MakeArray` "Non ho i soldi." "*Paga con il dollaro*" :!type "Text"))))
                  (switch `/Game/Blueprints/Components/Dialogues/E_DialogueState` _state_5
                    (:`NewEnumerator0`
                      (switch `int` _optionindex_2
                        (:`0`
                          (bind _state_6 (`self.AddDialogue` "Commesso" "E allora sparisci mocciosa." true (`|MakeArray` "Pff" :!type "Text")))
                          (switch `/Game/Blueprints/Components/Dialogues/E_DialogueState` _state_6
                            (:`NewEnumerator0`
                              (`self.RemoveDialogueProgress` 1)
                              (`self.CloseConversation`))))
                        (:`1`
                          (bind (_state_7 _optionindex_3) (`self.AddDialogue` "Commesso" "Moooolto bene" true (`|MakeArray` "Insomma? Le informazioni sul gatto?" "Mh. Ciao." :!type "Text")))
                          (switch `/Game/Blueprints/Components/Dialogues/E_DialogueState` _state_7
                            (:`NewEnumerator0`
                              (switch `int` _optionindex_3
                                (:`0`
                                  (bind _state_8 (`self.AddDialogue` "Commesso" "Non ho visto nessun gatto, solo teppistelli" true (`|MakeArray` "Maledetto bugiardo." :!type "Text")))
                                  (switch `/Game/Blueprints/Components/Dialogues/E_DialogueState` _state_8
                                    (:`NewEnumerator0`
                                      _)))
                                (:`1`
                                  _))
                              (bind _state_9 (`self.AddDialogue` "Commesso" "Alla prossima :)" true (`|MakeArray` "Pff" :!type "Text")))
                              (switch `/Game/Blueprints/Components/Dialogues/E_DialogueState` _state_9
                                (:`NewEnumerator0`
                                  (`self.SetDialogueTreeIndex` 1)
                                  (`self.CloseConversation`))))
                            (:`NewEnumerator1`
                              (`self.ProgressDialogueQuest` "BuyMilk" 1)
                              (`/Game/Blueprints/Components/AC_Inventory.RemoveFromInventory` (`/Game/Characters/MainCharacter/BP_MainCharacter.InventoryComponent` (`/Game/Blueprints/CommonFuntionLibrary.GetMyPlayerCharacter`)) "Dollaro" 1))))))))))))))
    (:`1`
      (bind (_state_10 _optionindex_4) (`self.AddDialogue` "Commesso" "Ti sei già dimenticata?" true (`|MakeArray` "Ridimmi del gatto." "Stavo solo vedendo se eri ancora sveglio." :!type "Text")))
      (switch `/Game/Blueprints/Components/Dialogues/E_DialogueState` _state_10
        (:`NewEnumerator0`
          (switch `int` _optionindex_4
            (:`0`
              (bind _state_11 (`self.AddDialogue` "Commesso" "Non ho visto nessun gatto, solo teppistelli" false (`|MakeArray` "" :!type "Text")))
              (switch `/Game/Blueprints/Components/Dialogues/E_DialogueState` _state_11
                (:`NewEnumerator0`
                  (`self.ClearDialogueProgress`)
                  (`self.CloseConversation`))))
            (:`1`
              (`self.ClearDialogueProgress`)
              (`self.CloseConversation`))))))))