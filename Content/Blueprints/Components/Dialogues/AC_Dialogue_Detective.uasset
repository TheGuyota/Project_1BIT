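; Dialogue component for the Detective NPC, who talks with a child searching for a cat while he hunts a "monster".
; A switch on DialogueTreeIndex stages chained AddDialogue calls, advancing through conversation or inventory clues that are then removed.
; Most stage endings relocate the NPC across the map.
; The Businessman global parameter switches to farewell dialogue from a threshold, and the Mostro parameter unlocks an extra question.
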(fn `Dialogue`
  (if (< (`self.QueryGlobalParameters` "Businessman") 4)
    (switch `int` (`self.DialogueTreeIndex`)
      (:`0`
        (bind _state (`self.AddDialogue` "Detective" "..." true (`|MakeArray` "Hey! Who are you?" :!type "Text")))
        (switch `/Game/Blueprints/Components/Dialogues/E_DialogueState` _state
          (:`NewEnumerator0`
            (bind _state_2 (`self.AddDialogue` "Detective" "... \nWho? Me?" true (`|MakeArray` "Yeah, who else?" :!type "Text")))
            (switch `/Game/Blueprints/Components/Dialogues/E_DialogueState` _state_2
              (:`NewEnumerator0`
                (bind _state_3 (`self.AddDialogue` "Detective" "Oh, I'm a detective. But don't tell anyone, kid. Wait, are you...? Oh yeah, I think I know your parents." true (`|MakeArray` "My parents? How?" :!type "Text")))
                (switch `/Game/Blueprints/Components/Dialogues/E_DialogueState` _state_3
                  (:`NewEnumerator0`
                    (bind _state_4 (`self.AddDialogue` "Detective" "Well, your mama once hired me to investigate on... Ah, nevermind, don't bother me, kid." true (`|MakeArray` "Hmm... Can you help me find my cat?" :!type "Text")))
                    (switch `/Game/Blueprints/Components/Dialogues/E_DialogueState` _state_4
                      (:`NewEnumerator0`
                        (bind _state_5 (`self.AddDialogue` "Detective" "I'm working right now, I got no time for this. I'm on the trails of a bloody monster. And that's why you should get back home. It's not safe for you." true (`|MakeArray` "Monsters? Do you see them too?" :!type "Text")))
                        (switch `/Game/Blueprints/Components/Dialogues/E_DialogueState` _state_5
                          (:`NewEnumerator0`
                            (bind _state_6 (`self.AddDialogue` "Detective" "Yeah kiddo, keep an eye on them. Monsters are everywhere. And so are good people. Like black and white... They mix up. It's a grey world, kiddo." false (`|MakeArray` "" :!type "Text")))
                            (switch `/Game/Blueprints/Components/Dialogues/E_DialogueState` _state_6
                              (:`NewEnumerator0`
                                (`/Game/Blueprints/NPCs/BP_NPC_Master.UpdateSelfLocation` (`/Game/Blueprints/CommonFuntionLibrary.GetOwnerNPC` self) (40.0 -420.0 150.0))
                                (`self.IncrementGlobalParameter` "Businessman")
                                (`self.SetDialogueTreeIndex` 1)
                                (`self.CloseConversation`))))))))))))))
      (:`1`
        (bind _state_7 (`self.AddDialogue` "Detective" "Hey. Didn't I tell you to go back home?" true (`|MakeArray` "I do HAVE to find my cat!" :!type "Text")))
        (switch `/Game/Blueprints/Components/Dialogues/E_DialogueState` _state_7
          (:`NewEnumerator0`
            (bind _state_8 (`self.AddDialogue` "Detective" "You're pretty determined, huh?" true (`|MakeArray` "I am!" :!type "Text")))
            (switch `/Game/Blueprints/Components/Dialogues/E_DialogueState` _state_8
              (:`NewEnumerator0`
                (bind (_state_9 _optionindex) (`self.AddDialogue` "Detective" "You're pretty determined, huh?" true (`|MakeArray` "What does that mean?" "I'll find my cat, no matter what!" :!type "Text")))
                (switch `/Game/Blueprints/Components/Dialogues/E_DialogueState` _state_9
                  (:`NewEnumerator0`
                    (switch `int` _optionindex
                      (:`0`
                        (bind _state_10 (`self.AddDialogue` "Detective" "The \"monsters\", girl. Be careful." true (`|MakeArray` "What a strange man." :!type "Text")))
                        (switch `/Game/Blueprints/Components/Dialogues/E_DialogueState` _state_10
                          (:`NewEnumerator0`
                            _)))
                      (:`1`
                        _))
                    (`/Game/Blueprints/NPCs/BP_NPC_Master.UpdateSelfLocation` (`/Game/Blueprints/CommonFuntionLibrary.GetOwnerNPC` self) (-2120.0 1930.0 150.0))
                    (`self.SetDialogueTreeIndex` 2)
                    (`self.CloseConversation`))))))))
      (:`2`
        (if (`.bIsFound` (`/Game/Blueprints/Components/AC_Inventory.QueryInventory` (`/Game/Characters/MainCharacter/BP_MainCharacter.InventoryComponent` (`/Game/Blueprints/CommonFuntionLibrary.GetMyPlayerCharacter`)) "Chiavi"))
          (bind _state_11 (`self.AddDialogue` "Detective" "You again huh?" true (`|MakeArray` "I found these keys." :!type "Text")))
          (switch `/Game/Blueprints/Components/Dialogues/E_DialogueState` _state_11
            (:`NewEnumerator0`
              (bind _state_12 (`self.AddDialogue` "Detective" "Huh? Could these be... His house keys?" true (`|MakeArray` "Is it a good clue?" :!type "Text")))
              (switch `/Game/Blueprints/Components/Dialogues/E_DialogueState` _state_12
                (:`NewEnumerator0`
                  (bind _state_13 (`self.AddDialogue` "Detective" "Could be... If I had some more proof." false (`|MakeArray` "" :!type "Text")))
                  (switch `/Game/Blueprints/Components/Dialogues/E_DialogueState` _state_13
                    (:`NewEnumerator0`
                      (`/Game/Blueprints/Components/AC_Inventory.RemoveFromInventory` (`/Game/Characters/MainCharacter/BP_MainCharacter.InventoryComponent` (`/Game/Blueprints/CommonFuntionLibrary.GetMyPlayerCharacter`)) "Chiavi" 1)
                      (`self.SetDialogueTreeIndex` 3)))))))
          (else
            (bind _state_14 (`self.AddDialogue` "Detective" "You again huh?" true (`|MakeArray` "Just searching for my cat!" :!type "Text")))
            (switch `/Game/Blueprints/Components/Dialogues/E_DialogueState` _state_14
              (:`NewEnumerator0`
                (bind _state_15 (`self.AddDialogue` "Detective" "I see." true (`|MakeArray` "See ya." :!type "Text")))
                (switch `/Game/Blueprints/Components/Dialogues/E_DialogueState` _state_15
                  (:`NewEnumerator0`
                    (`self.ClearDialogueProgress`)
                    (`self.CloseConversation`))))))))
      (:`3`
        (if (`.bIsFound` (`/Game/Blueprints/Components/AC_Inventory.QueryInventory` (`/Game/Characters/MainCharacter/BP_MainCharacter.InventoryComponent` (`/Game/Blueprints/CommonFuntionLibrary.GetMyPlayerCharacter`)) "Orologio"))
          (bind _state_16 (`self.AddDialogue` "Detective" "Did you find anything else?" true (`|MakeArray` "I found a shiny watch!" :!type "Text")))
          (switch `/Game/Blueprints/Components/Dialogues/E_DialogueState` _state_16
            (:`NewEnumerator0`
              (bind _state_17 (`self.AddDialogue` "Detective" "...Good heavens... Where did you even find this? I..." true (`|MakeArray` "So, the monster likes shiny things?" :!type "Text")))
              (switch `/Game/Blueprints/Components/Dialogues/E_DialogueState` _state_17
                (:`NewEnumerator0`
                  (bind _state_18 (`self.AddDialogue` "Detective" "Like I said... It's a grey world. Black and white cross endlessly." false (`|MakeArray` "I hope the monster didn't find my kitty..." :!type "Text")))
                  (switch `/Game/Blueprints/Components/Dialogues/E_DialogueState` _state_18
                    (:`NewEnumerator0`
                      (`/Game/Blueprints/Components/AC_Inventory.RemoveFromInventory` (`/Game/Characters/MainCharacter/BP_MainCharacter.InventoryComponent` (`/Game/Blueprints/CommonFuntionLibrary.GetMyPlayerCharacter`)) "Orologio" 1)
                      (`/Game/Blueprints/NPCs/BP_NPC_Master.UpdateSelfLocation` (`/Game/Blueprints/CommonFuntionLibrary.GetOwnerNPC` self) (-3930.0 -2780.0 150.0))
                      (`self.SetDialogueTreeIndex` 4)
                      (`self.CloseConversation`)))))))
          (else
            (bind _state_19 (`self.AddDialogue` "Detective" "Did you find anything else?" true (`|MakeArray` "Nothing..." :!type "Text")))
            (switch `/Game/Blueprints/Components/Dialogues/E_DialogueState` _state_19
              (:`NewEnumerator0`
                (`self.ClearDialogueProgress`)
                (`self.CloseConversation`))))))
      (:`4`
        (bind _state_20 (`self.AddDialogue` "Detective" "Still wandering around, huh? Looks like I got some competition in this town, hehe.  \nDid you find your cat already?" true (`|MakeArray` "Not yet, sadly." :!type "Text")))
        (switch `/Game/Blueprints/Components/Dialogues/E_DialogueState` _state_20
          (:`NewEnumerator0`
            (bind (_state_21 _optionindex_2) (`self.AddDialogue` "Detective" "I see... I wish you the best of luck finding clues." true (select `bool` (>= (`.Quantity` (`self.QueryGlobalParameters` "Mostro")) 1) :`false` (`|MakeArray` "Who hired you?" :!type "Text") :`true` (`|MakeArray` "Who hired you?" "Can you tell me more about the monsters?" :!type "Text"))))
            (switch `/Game/Blueprints/Components/Dialogues/E_DialogueState` _state_21
              (:`NewEnumerator0`
                (switch `int` _optionindex_2
                  (:`0`
                    (bind _state_22 (`self.AddDialogue` "Detective" "Can't tell you... Professional secret." true (`|MakeArray` "Can I hire you to find my cat?" :!type "Text")))
                    (switch `/Game/Blueprints/Components/Dialogues/E_DialogueState` _state_22
                      (:`NewEnumerator0`
                        (bind _state_23 (`self.AddDialogue` "Detective" "Haha! ...Ahhhh, to be young again!" true (`|MakeArray` "Hey, I love my kitty!" :!type "Text")))
                        (switch `/Game/Blueprints/Components/Dialogues/E_DialogueState` _state_23
                          (:`NewEnumerator0`
                            _)))))
                  (:`1`
                    (bind _state_24 (`self.AddDialogue` "Detective" "Ah, monsters... They are just like us. More like me, maybe. We walk close to them. We talk with them. And yet, they are the ones who fear us. Believe me, you don't want to know about them." true (`|MakeArray` "They scare me sometimes!" :!type "Text")))
                    (switch `/Game/Blueprints/Components/Dialogues/E_DialogueState` _state_24
                      (:`NewEnumerator0`
                        (bind _state_25 (`self.AddDialogue` "Detective" "You gotta learn how to act, kiddo. Kids your age are beacons of innocence. A weak light in our society. But a light nonetheless." true (`|MakeArray` "Yes! The light!" :!type "Text")))
                        (switch `/Game/Blueprints/Components/Dialogues/E_DialogueState` _state_25
                          (:`NewEnumerator0`
                            _))))))
                (`/Game/Blueprints/NPCs/BP_NPC_Master.UpdateSelfLocation` (`/Game/Blueprints/CommonFuntionLibrary.GetOwnerNPC` self) (860.0 -2910.0 150.0))
                (`self.SetDialogueTreeIndex` 5)
                (`self.CloseConversation`))))))
      (:`5`
        (bind _state_26 (`self.AddDialogue` "Detective" "Tell me youngster... What makes you wander at this time of the night with all this energy?" true (`|MakeArray` "My cat, duh!" :!type "Text")))
        (switch `/Game/Blueprints/Components/Dialogues/E_DialogueState` _state_26
          (:`NewEnumerator0`
            (bind _state_27 (`self.AddDialogue` "Detective" "Well, maybe it will come back tomorrow, don't you think so?" true (`|MakeArray` "Gah! You wouldn't understand!" :!type "Text")))
            (switch `/Game/Blueprints/Components/Dialogues/E_DialogueState` _state_27
              (:`NewEnumerator0`
                (`/Game/Blueprints/NPCs/BP_NPC_Master.UpdateSelfLocation` (`/Game/Blueprints/CommonFuntionLibrary.GetOwnerNPC` self) (-2370.0 3230.0 150.0))
                (`self.SetDialogueTreeIndex` 6)
                (`self.CloseConversation`))))))
      (:`6`
        (if (`.bIsFound` (`/Game/Blueprints/Components/AC_Inventory.QueryInventory` (`/Game/Characters/MainCharacter/BP_MainCharacter.InventoryComponent` (`/Game/Blueprints/CommonFuntionLibrary.GetMyPlayerCharacter`)) "Bende"))
          (bind _state_28 (`self.AddDialogue` "Detective" "..." true (`|MakeArray` "I found this bandage!" :!type "Text")))
          (switch `/Game/Blueprints/Components/Dialogues/E_DialogueState` _state_28
            (:`NewEnumerator0`
              (bind _state_29 (`self.AddDialogue` "Detective" "Huh? Hmm... Someone used it to clean blood on their hands." true (`|MakeArray` "Is it a good clue?" :!type "Text")))
              (switch `/Game/Blueprints/Components/Dialogues/E_DialogueState` _state_29
                (:`NewEnumerator0`
                  (bind _state_30 (`self.AddDialogue` "Detective" "Could be... If I had some more proof." false (`|MakeArray` "" :!type "Text")))
                  (switch `/Game/Blueprints/Components/Dialogues/E_DialogueState` _state_30
                    (:`NewEnumerator0`
                      (`/Game/Blueprints/Components/AC_Inventory.RemoveFromInventory` (`/Game/Characters/MainCharacter/BP_MainCharacter.InventoryComponent` (`/Game/Blueprints/CommonFuntionLibrary.GetMyPlayerCharacter`)) "Bende" 1)
                      (`self.SetDialogueTreeIndex` 7)
                      (`self.CloseConversation`)))))))
          (else
            (bind _state_31 (`self.AddDialogue` "Detective" "..." true (`|MakeArray` "Found anything sir?" :!type "Text")))
            (switch `/Game/Blueprints/Components/Dialogues/E_DialogueState` _state_31
              (:`NewEnumerator0`
                (bind _state_32 (`self.AddDialogue` "Detective" "I'm just a few steps behind him... Every bit, every clue... It's all coming together." true (`|MakeArray` "Same as me with my cat!" :!type "Text")))
                (switch `/Game/Blueprints/Components/Dialogues/E_DialogueState` _state_32
                  (:`NewEnumerator0`
                    (`self.ClearDialogueProgress`)
                    (`self.CloseConversation`))))))))
      (:`7`
        (if (`.bIsFound` (`/Game/Blueprints/Components/AC_Inventory.QueryInventory` (`/Game/Characters/MainCharacter/BP_MainCharacter.InventoryComponent` (`/Game/Blueprints/CommonFuntionLibrary.GetMyPlayerCharacter`)) "Bottiglia"))
          (bind _state_33 (`self.AddDialogue` "Detective" "Come on kiddo, go home. It's getting real late now." true (`|MakeArray` "The guy at the park gave me this." :!type "Text")))
          (switch `/Game/Blueprints/Components/Dialogues/E_DialogueState` _state_33
            (:`NewEnumerator0`
              (bind _state_34 (`self.AddDialogue` "Detective" "What's so special about it?" true (`|MakeArray` "A crazy guy threw it to him!" :!type "Text")))
              (switch `/Game/Blueprints/Components/Dialogues/E_DialogueState` _state_34
                (:`NewEnumerator0`
                  (bind _state_35 (`self.AddDialogue` "Detective" "Could it be...? Yes, yes, it all makes sense now." false (`|MakeArray` "Was it the monster?" :!type "Text")))
                  (switch `/Game/Blueprints/Components/Dialogues/E_DialogueState` _state_35
                    (:`NewEnumerator0`
                      (bind _state_36 (`self.AddDialogue` "Detective" "Quite possibly, yes. And wash your hands when you get home." false (`|MakeArray` "Do you think the monsters killed my cat?" :!type "Text")))
                      (switch `/Game/Blueprints/Components/Dialogues/E_DialogueState` _state_36
                        (:`NewEnumerator0`
                          (bind _state_37 (`self.AddDialogue` "Detective" "No, I'm sure they didn't. Sorry kiddo, I must go now. Your help was so useful to my investigation you deserve a medal." false (`|MakeArray` "" :!type "Text")))
                          (switch `/Game/Blueprints/Components/Dialogues/E_DialogueState` _state_37
                            (:`NewEnumerator0`
                              (bind _state_38 (`self.AddDialogue` "Detective" "For now... Goodbye." true (`|MakeArray` "See ya Mr. Detective." :!type "Text")))
                              (switch `/Game/Blueprints/Components/Dialogues/E_DialogueState` _state_38
                                (:`NewEnumerator0`
                                  (`/Game/Blueprints/Components/AC_Inventory.RemoveFromInventory` (`/Game/Characters/MainCharacter/BP_MainCharacter.InventoryComponent` (`/Game/Blueprints/CommonFuntionLibrary.GetMyPlayerCharacter`)) "Bottiglia" 1)
                                  (`/Game/Blueprints/NPCs/BP_NPC_Master.UpdateSelfLocation` (`/Game/Blueprints/CommonFuntionLibrary.GetOwnerNPC` self) (21460.0 3230.0 150.0))
                                  (`self.CloseConversation`)))))))))))))
          (else
            (bind _state_39 (`self.AddDialogue` "Detective" "Come on kiddo, go home. It's getting real late now." true (`|MakeArray` "No! I still wanna find my cat!" :!type "Text")))
            (switch `/Game/Blueprints/Components/Dialogues/E_DialogueState` _state_39
              (:`NewEnumerator0`
                (`self.ClearDialogueProgress`)
                (`self.CloseConversation`)))))))
    (elif (> (`self.DialogueTreeIndex`) 0)
      (bind _state_40 (`self.AddDialogue` "Detective" "Oh hey, it's you again kid. Did you find your cat already?" true (`|MakeArray` "No, I didn't find it yet... What about you? " :!type "Text")))
      (switch `/Game/Blueprints/Components/Dialogues/E_DialogueState` _state_40
        (:`NewEnumerator0`
          (bind _state_41 (`self.AddDialogue` "Detective" "Unfortunately, no. All the clues I found made me realitze it's too lte..." true (`|MakeArray` "I'm sure when we find my cat, we'llfind the monster as well" :!type "Text")))
          (switch `/Game/Blueprints/Components/Dialogues/E_DialogueState` _state_41
            (:`NewEnumerator0`
              (bind _state_42 (`self.AddDialogue` "Detective" "Hope so, little girl, hope so." false (`|MakeArray` "" :!type "Text")))
              (switch `/Game/Blueprints/Components/Dialogues/E_DialogueState` _state_42
                (:`NewEnumerator0`
                  (`/Game/Blueprints/NPCs/BP_NPC_Master.UpdateSelfLocation` (`/Game/Blueprints/CommonFuntionLibrary.GetOwnerNPC` self) (21460.0 3230.0 150.0))
                  (`self.CloseConversation`)))))))
      (else
        (bind _state_43 (`self.AddDialogue` "Detective" "Hey there, it's pretty late to stay here now, you should be home right now." true (`|MakeArray` "Who are you?" :!type "Text")))
        (switch `/Game/Blueprints/Components/Dialogues/E_DialogueState` _state_43
          (:`NewEnumerator0`
            (bind _state_44 (`self.AddDialogue` "Detective" "I'm... Nevermind. I'm nobody. Do like me, go home and get some sleep." false (`|MakeArray` "" :!type "Text")))
            (switch `/Game/Blueprints/Components/Dialogues/E_DialogueState` _state_44
              (:`NewEnumerator0`
                (`/Game/Blueprints/NPCs/BP_NPC_Master.UpdateSelfLocation` (`/Game/Blueprints/CommonFuntionLibrary.GetOwnerNPC` self) (21460.0 3230.0 150.0))
                (`self.CloseConversation`)))))))))