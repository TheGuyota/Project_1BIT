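; Dialogue component for the Granny NPC, driving her lost-glasses fetch quest and later hints about a cat.
; Branches on whether the player carries GrannyGlasses, then on DialogueTreeIndex to pick the Italian lines and reply options.
; Accepting the request adds GrannyQuest01; handing over the glasses removes the item, progresses the objective and swaps her sprite.
; Outcomes advance the tree index, while refusals clear dialogue progress.
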(fn `Dialogue`
  (if (`self.GetPlayerInventoryItem` "GrannyGlasses")
    (switch `int` (`self.DialogueTreeIndex`)
      (:`0`
        (bind (_state _optionindex) (`self.AddDialogue` "Granny" "Hey ma... quelli... quelli sono i miei occhiali?..." true (`|MakeArray` "Li ho trovati per terra, prendili..." "No. Sono miei." :!type "Text")))
        (switch `/Game/Blueprints/Components/Dialogues/E_DialogueState` _state
          (:`NewEnumerator0`
            (switch `int` _optionindex
              (:`0`
                (bind _state_2 (`self.AddDialogue` "Granny" "Il tempo di mettermeli" true (`|MakeArray` "Va bene" :!type "Text")))
                (switch `/Game/Blueprints/Components/Dialogues/E_DialogueState` _state_2
                  (:`NewEnumerator0`
                    (`/Game/Blueprints/NPCs/BP_NPC_Master.UpdateDialogueSprite` (`/Game/Blueprints/CommonFuntionLibrary.GetOwnerNPC` self) "/Game/Characters/DialogueCharacters/NPC_Vecchia_B.NPC_Vecchia_B")
                    (`/Game/Blueprints/Components/AC_Inventory.RemoveFromInventory` (`/Game/Characters/MainCharacter/BP_MainCharacter.InventoryComponent` (`/Game/Blueprints/CommonFuntionLibrary.GetMyPlayerCharacter`)) "GrannyGlasses" 1)
                    (`self.ProgressDialogueQuest` "GrannyGlasses" 1)
                    (`self.SetDialogueTreeIndex` 2)
                    (`self.CloseConversation`))))
              (:`1`
                (bind _state_3 (`self.AddDialogue` "Granny" "*Maledetta mocciosa...* Sparisci allora!" true (`|MakeArray` "*Lascia la conversazione*" :!type "Text")))
                (switch `/Game/Blueprints/Components/Dialogues/E_DialogueState` _state_3
                  (:`NewEnumerator0`
                    (`self.ClearDialogueProgress`)
                    (`self.CloseConversation`))))))))
      (:`1`
        (bind (_state_4 _optionindex_2) (`self.AddDialogue` "Granny" "LI HAI TROVATI GRAZIE!" true (`|MakeArray` "Li ho trovati per terra..." "No, non sono i tuoi occhiali!" :!type "Text")))
        (switch `/Game/Blueprints/Components/Dialogues/E_DialogueState` _state_4
          (:`NewEnumerator0`
            (switch `int` _optionindex_2
              (:`0`
                (`/Game/Blueprints/NPCs/BP_NPC_Master.UpdateDialogueSprite` (`/Game/Blueprints/CommonFuntionLibrary.GetOwnerNPC` self) "/Game/Characters/DialogueCharacters/NPC_Vecchia_B.NPC_Vecchia_B")
                (`/Game/Blueprints/Components/AC_Inventory.RemoveFromInventory` (`/Game/Characters/MainCharacter/BP_MainCharacter.InventoryComponent` (`/Game/Blueprints/CommonFuntionLibrary.GetMyPlayerCharacter`)) "GrannyGlasses" 1)
                (`self.ProgressDialogueQuest` "GrannyGlasses" 1)
                (`self.SetDialogueTreeIndex` 2)
                (`self.CloseConversation`))
              (:`1`
                (bind _state_5 (`self.AddDialogue` "Granny" "Ugh... Va bene..." true (`|MakeArray` "*Lascia la conversazione*" :!type "Text")))
                (switch `/Game/Blueprints/Components/Dialogues/E_DialogueState` _state_5
                  (:`NewEnumerator0`
                    (`self.ClearDialogueProgress`)
                    (`self.CloseConversation`)))))))))
    (else
      (switch `int` (`self.DialogueTreeIndex`)
        (:`0`
          (bind (_state_6 _optionindex_3) (`self.AddDialogue` "Granny" "Ti prego piccina aiutami a trovare i miei occhiali.." true (`|MakeArray` "Va bene nonnina" "Ho altro da fare..." :!type "Text")))
          (switch `/Game/Blueprints/Components/Dialogues/E_DialogueState` _state_6
            (:`NewEnumerator0`
              (switch `int` _optionindex_3
                (:`0`
                  (bind _state_7 (`self.AddDialogue` "Granny" "GRAZIE! GRAZIE!" true (`|MakeArray` "*Lascia la conversazione*" :!type "Text")))
                  (switch `/Game/Blueprints/Components/Dialogues/E_DialogueState` _state_7
                    (:`NewEnumerator0`
                      (`self.AddNewQuest` "GrannyQuest01")
                      (`self.SetDialogueTreeIndex` 1)
                      (`self.CloseConversation`))))
                (:`1`
                  (bind _state_8 (`self.AddDialogue` "Granny" "Ugh... Va bene..." true (`|MakeArray` "*Lascia la conversazione*" :!type "Text")))
                  (switch `/Game/Blueprints/Components/Dialogues/E_DialogueState` _state_8
                    (:`NewEnumerator0`
                      (`self.ClearDialogueProgress`)
                      (`self.CloseConversation`))))))))
        (:`1`
          (bind _state_9 (`self.AddDialogue` "Granny" "Ancora niente eh..." true (`|MakeArray` "*Allontanati*" :!type "Text")))
          (switch `/Game/Blueprints/Components/Dialogues/E_DialogueState` _state_9
            (:`NewEnumerator0`
              (`self.ClearDialogueProgress`)
              (`self.CloseConversation`))))
        (:`2`
          (bind _state_10 (`self.AddDialogue` "Granny" "Non so dove sia il gatto ihihih... Ma qualcosa prima mi ha fatto spaventare a morte ihihih..." true (`|MakeArray` "...la ringrazio..." :!type "Text")))
          (switch `/Game/Blueprints/Components/Dialogues/E_DialogueState` _state_10
            (:`NewEnumerator0`
              (`self.ClearDialogueProgress`)
              (`self.SetDialogueTreeIndex` 3)
              (`self.CloseConversation`))))
        (:`3`
          (bind _state_11 (`self.AddDialogue` "Granny" "ihihih... Ti ho già detto che non so dove sia il gatto ihihih... " true (`|MakeArray` "*Allontanati*" :!type "Text")))
          (switch `/Game/Blueprints/Components/Dialogues/E_DialogueState` _state_11
            (:`NewEnumerator0`
              (`self.ClearDialogueProgress`)
              (`self.CloseConversation`))))))))

(fn `ProgressDialogue`
  (`parent.ProgressDialogue`))