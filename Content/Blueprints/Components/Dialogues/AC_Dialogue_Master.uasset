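; Base dialogue component that runs branching conversations in a W_Dialogue widget while pausing the game.
; Child components override the empty Dialogue function, which replays from the top after each choice.
; AddDialogue returns recorded choices from the DialogueProgress map and displays the first unanswered line, so clearing or removing entries rewinds the conversation.
; Helpers let dialogue query or change player inventory, quests and GameInstance global parameters, including side-quest counters.
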(event `self.ReceiveBeginPlay`
  (bind _asbp_default_game_instance (cast `/Game/Blueprints/Core/BP_DefaultGameInstance` (`GameplayStatics.GetGameInstance`)))
  (set `self.GameInstanceRef` _asbp_default_game_instance)
  (bind _asbp_in_game_controller (cast `/Game/Blueprints/Core/InGameController/BP_InGameController` (`GameplayStatics.GetPlayerController` 0)))
  (set `self.InGameControllerRef` _asbp_in_game_controller))

(fn `AddDialogue`
  (params (Speaker :type Text) (Dialogue :type Text) (bHasOptions :type Boolean :default true) (OptionsText :type "Array of Text"))
  (returns (State :type "/Game/Blueprints/Components/Dialogues/E_DialogueState Enum") (OptionIndex :type Integer))
  (bind (_value _returnvalue) (`BlueprintMapLibrary.Map_Find` (`self.DialogueProgress`) (`self.DialogueIndex`)))
  (`/Engine/EditorBlueprintResources/StandardMacros.IncrementInt` (`self.DialogueIndex`)
    (:`  `
      (if _returnvalue
        (return "NewEnumerator0" _value)
        (else
          (`/Game/Widgets/DialogueSystem/W_Dialogue.UpdateDialogueText` (`self.DialogueWidget`) (`self.DialogueIndex`) (`local.Speaker`) (`local.Dialogue`) (`local.bHasOptions`) (`local.OptionsText`))
          (return "NewEnumerator1" _value))))))

(fn `AddNewQuest`
  (params (QuestID :type Name))
  (if (not (`/Game/Blueprints/QuestSystem/AC_QuestLog.QueryActiveQuest` (`/Game/Characters/MainCharacter/BP_MainCharacter.QuestLogComponent` (`/Game/Blueprints/CommonFuntionLibrary.GetMyPlayerCharacter`)) QuestID))
    (`/Game/Blueprints/QuestSystem/AC_QuestLog.AddNewQuest` (`/Game/Characters/MainCharacter/BP_MainCharacter.QuestLogComponent` (`/Game/Blueprints/CommonFuntionLibrary.GetMyPlayerCharacter`)) (`local.QuestID`))
    (return)))

(fn `CheckAndUpdateSideQuest`
  (if (== (`.Quantity` (`self.QueryGlobalParameters` "SideQuest")) 0)
    (`self.IncrementGlobalParameter` "Businessman")
    (`self.IncrementGlobalParameter` "SideQuest")
    (return)
    (else
      (`self.IncrementGlobalParameter` "SideQuest")
      (return))))

(fn `ClearDialogueProgress`
  (`BlueprintMapLibrary.Map_Clear` (`self.DialogueProgress`))
  (return))

(fn `CloseConversation`
  (`/Game/Widgets/DialogueSystem/W_Dialogue.Deactivate` (`self.DialogueWidget`))
  (set `self.DialogueWidget` null)
  (message `/Game/Blueprints/Interfaces/BPI_Interaction.ConversationClosed` (`self.GetOwner`)))

(fn `Dialogue`)

(fn `GetPlayerInventoryItem`
  (params (ItemName :type Name))
  (returns (bIsFound :type Boolean) (Quantity :type Integer))
  (bind (_value _bisfound) (`/Game/Blueprints/Components/AC_Inventory.QueryInventory` (`/Game/Characters/MainCharacter/BP_MainCharacter.InventoryComponent` (`/Game/Blueprints/CommonFuntionLibrary.GetMyPlayerCharacter`)) ItemName))
  (return _bisfound _value))

(fn `IncrementGlobalParameter`
  (params (Name :type String))
  (bind _globalparameters (`/Game/Blueprints/Core/BP_DefaultGameInstance.GlobalParameters` (`self.GameInstanceRef`)))
  (`BlueprintMapLibrary.Map_Add` _globalparameters Name (+ (`BlueprintMapLibrary.Map_Find` (`/Game/Blueprints/Core/BP_DefaultGameInstance.GlobalParameters` (`self.GameInstanceRef`)) Name) 1))
  (`/Game/Blueprints/Core/BP_DefaultGameInstance.OnGlobalParameterUpdated` (`self.GameInstanceRef`) (`local.Name`) (`BlueprintMapLibrary.Map_Find` _globalparameters (`local.Name`)))
  (return))

(fn `ProgressDialogue`
  (set `self.DialogueIndex` -1)
  (`self.Dialogue`))

(fn `ProgressDialogueQuest`
  (params (ObjectiveID :type String) (Value :type Integer))
  (`/Game/Characters/MainCharacter/BP_MainCharacter.OnObjectiveIDCalled` (`/Game/Blueprints/CommonFuntionLibrary.GetMyPlayerCharacter`) ObjectiveID Value)
  (return))

(fn `QueryGlobalParameters`
  (params (Name :type String))
  (returns (bIsFound :type Boolean) (Quantity :type Integer))
  (bind (_value _returnvalue) (`BlueprintMapLibrary.Map_Find` (`/Game/Blueprints/Core/BP_DefaultGameInstance.GlobalParameters` (`self.GameInstanceRef`)) (`local.Name`)))
  (return _returnvalue _value))

(fn `RemoveDialogueProgress`
  (params (ProgressSteps :type Integer))
  (for _index (range (+ ProgressSteps 1))
    (`BlueprintMapLibrary.Map_Remove` (`self.DialogueProgress`) (- (`self.DialogueIndex`) _index))))

(fn `RemovePlayerInventoryItem`
  (params (ItemName :type Name) (QuantityToRemove :type Integer))
  (`/Game/Blueprints/Components/AC_Inventory.RemoveFromInventory` (`/Game/Characters/MainCharacter/BP_MainCharacter.InventoryComponent` (`/Game/Blueprints/CommonFuntionLibrary.GetMyPlayerCharacter`)) ItemName QuantityToRemove)
  (return))

(fn `SetDialogueTreeIndex`
  (params (DialogueTreeIndex :type Integer))
  (set `self.DialogueTreeIndex` DialogueTreeIndex)
  (`self.ClearDialogueProgress`))

(fn `StartConversation`
  (bind _returnvalue (`|CreateWidget` "/Game/Widgets/DialogueSystem/W_Dialogue.W_Dialogue_C" null (`self.DialogueBG`) (`self.LeftSpeaker`) (`self.RightSpeaker`) self))
  (`UserWidget.AddToViewport` _returnvalue 0)
  (set `self.DialogueWidget` _returnvalue)
  (`self.ProgressDialogue`)
  (`WidgetBlueprintLibrary.SetInputMode_UIOnlyEx` (`self.InGameControllerRef`) null "DoNotLock" true)
  (`GameplayStatics.SetGamePaused` true))

(fn `UpdateGlobalParameter`
  (params (Name :type String) (Value :type Integer))
  (`BlueprintMapLibrary.Map_Add` (`/Game/Blueprints/Core/BP_DefaultGameInstance.GlobalParameters` (`self.GameInstanceRef`)) Name Value)
  (`/Game/Blueprints/Core/BP_DefaultGameInstance.OnGlobalParameterUpdated` (`self.GameInstanceRef`) (`local.Name`) (`BlueprintMapLibrary.Map_Find` (`/Game/Blueprints/Core/BP_DefaultGameInstance.GlobalParameters` (`self.GameInstanceRef`)) (`local.Name`)))
  (return))

(fn `UpdateSelectedOption`
  (params (ProgressIndex :type "Integer (by ref)") (OptionIndex :type "Integer (by ref)"))
  (`BlueprintMapLibrary.Map_Add` (`self.DialogueProgress`) ProgressIndex OptionIndex)
  (`self.ProgressDialogue`))