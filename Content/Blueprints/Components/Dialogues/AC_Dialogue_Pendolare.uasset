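; Dialogue component for the commuter NPC "Pendolare", who trades a cat sighting clue for a lost ticket.
; A tree index selects the conversation, built from nested AddDialogue calls that branch on state and chosen option.
; The first tree offers the ticket only if the inventory holds it, then advances the quest objective, removes the item and switches trees.
; The second tree repeats the clue or closes the conversation.
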(fn `Dialogue`
  (switch `int` (`self.DialogueTreeIndex`)
    (:`0`
      (bind (_state _optionindex) (`self.AddDialogue` "Pendolare" "Dimmi ragazzina." true (select `bool` (`.bIsFound` (`/Game/Blueprints/Components/AC_Inventory.QueryInventory` (`/Game/Characters/MainCharacter/BP_MainCharacter.InventoryComponent` (`/Game/Blueprints/CommonFuntionLibrary.GetMyPlayerCharacter`)) "Biglietto")) :`false` (`|MakeArray` "Non ho nulla da dirti..." :!type "Text") :`true` (`|MakeArray` "Non ho nulla da dirti..." "*Dai il biglietto*" :!type "Text"))))
      (switch `/Game/Blueprints/Components/Dialogues/E_DialogueState` _state
        (:`NewEnumerator0`
          (switch `int` _optionindex
            (:`0`
              (bind _state_2 (`self.AddDialogue` "Pendolare" "Torna a casa ragazzina." false (`|MakeArray` "" :!type "Text")))
              (switch `/Game/Blueprints/Components/Dialogues/E_DialogueState` _state_2
                (:`NewEnumerator0`
                  (`self.ClearDialogueProgress`)
                  (`self.CloseConversation`))))
            (:`1`
              (bind _state_3 (`self.AddDialogue` "Pendolare" "Davvero lo hai trovato..." true (`|MakeArray` "Sapevo che era suo eheheh" :!type "Text")))
              (switch `/Game/Blueprints/Components/Dialogues/E_DialogueState` _state_3
                (:`NewEnumerator0`
                  (bind _state_4 (`self.AddDialogue` "Barbone" "Ho visto un gatto che correva mentre inseguiva un topo!" false (`|MakeArray` "" :!type "Text")))
                  (switch `/Game/Blueprints/Components/Dialogues/E_DialogueState` _state_4
                    (:`NewEnumerator0`
                      (`self.SetDialogueTreeIndex` 1)
                      (`self.CloseConversation`))))
                (:`NewEnumerator1`
                  (`self.ProgressDialogueQuest` "DaiBiglietto" 1)
                  (`/Game/Blueprints/Components/AC_Inventory.RemoveFromInventory` (`/Game/Characters/MainCharacter/BP_MainCharacter.InventoryComponent` (`/Game/Blueprints/CommonFuntionLibrary.GetMyPlayerCharacter`)) "Biglietto" 1))))))))
    (:`1`
      (bind (_state_5 _optionindex_2) (`self.AddDialogue` "Pendolare" "Hey ragazzina sei ancora te?" true (`|MakeArray` "Mi scusi può ripetermi dove ha visto il gattino..." "Sta ancora aspettando l'autobus? *Vattene*" :!type "Text")))
      (switch `/Game/Blueprints/Components/Dialogues/E_DialogueState` _state_5
        (:`NewEnumerator0`
          (switch `int` _optionindex_2
            (:`0`
              (bind _state_6 (`self.AddDialogue` "Pendolare" "Ho visto un gatto che correva mentre inseguiva un topo!" false (`|MakeArray` "" :!type "Text")))
              (switch `/Game/Blueprints/Components/Dialogues/E_DialogueState` _state_6
                (:`NewEnumerator0`
                  (`self.ClearDialogueProgress`)
                  (`self.CloseConversation`))))
            (:`1`
              (`self.ClearDialogueProgress`)
              (`self.CloseConversation`))))))))