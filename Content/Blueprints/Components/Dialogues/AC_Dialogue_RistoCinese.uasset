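; Dialogue component for the RistoCinese NPC, who can receive cigarettes from the player and be asked about a missing cat.
; The first tree offers the hand-over option only if the inventory query finds "Sigarette"; choosing it progresses the DaiSigarette quest objective and removes one item.
; Finishing that exchange switches DialogueTreeIndex to a repeat tree, where the player can re-ask about the cat or leave.
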(fn `Dialogue`
  (switch `int` (`self.DialogueTreeIndex`)
    (:`0`
      (bind (_state _optionindex) (`self.AddDialogue` "RistoCinese" "Cosa vuoi lagazzina?" true (select `bool` (`.bIsFound` (`/Game/Blueprints/Components/AC_Inventory.QueryInventory` (`/Game/Characters/MainCharacter/BP_MainCharacter.InventoryComponent` (`/Game/Blueprints/CommonFuntionLibrary.GetMyPlayerCharacter`)) "Sigarette")) :`false` (`|MakeArray` "Non posso aiutarti" :!type "Text") :`true` (`|MakeArray` "Non posso aiutarti" "*Dai le sigarette*" :!type "Text"))))
      (switch `/Game/Blueprints/Components/Dialogues/E_DialogueState` _state
        (:`NewEnumerator0`
          (switch `int` _optionindex
            (:`0`
              (bind _state_2 (`self.AddDialogue` "RistoCinese" "E allora spalisci." false (`|MakeArray` "" :!type "Text")))
              (switch `/Game/Blueprints/Components/Dialogues/E_DialogueState` _state_2
                (:`NewEnumerator0`
                  (`self.ClearDialogueProgress`)
                  (`self.CloseConversation`))))
            (:`1`
              (bind _state_3 (`self.AddDialogue` "RistoCinese" "Grazie lagazzina" true (`|MakeArray` "Sai qualcosa del mio gatto?" :!type "Text")))
              (switch `/Game/Blueprints/Components/Dialogues/E_DialogueState` _state_3
                (:`NewEnumerator0`
                  (bind _state_4 (`self.AddDialogue` "RistoCinese" "Non ho visto il gatto" false (`|MakeArray` "" :!type "Text")))
                  (switch `/Game/Blueprints/Components/Dialogues/E_DialogueState` _state_4
                    (:`NewEnumerator0`
                      (`self.SetDialogueTreeIndex` 1)
                      (`self.CloseConversation`))))
                (:`NewEnumerator1`
                  (`self.ProgressDialogueQuest` "DaiSigarette" 1)
                  (`/Game/Blueprints/Components/AC_Inventory.RemoveFromInventory` (`/Game/Characters/MainCharacter/BP_MainCharacter.InventoryComponent` (`/Game/Blueprints/CommonFuntionLibrary.GetMyPlayerCharacter`)) "Sigarette" 1))))))))
    (:`1`
      (bind (_state_5 _optionindex_2) (`self.AddDialogue` "RistoCinese" "Ola cosa vuoi?" true (`|MakeArray` "Senti puoi ridirmi cosa sapevi del gatto?..." "*Voltati e vattene*" :!type "Text")))
      (switch `/Game/Blueprints/Components/Dialogues/E_DialogueState` _state_5
        (:`NewEnumerator0`
          (switch `int` _optionindex_2
            (:`0`
              (bind _state_6 (`self.AddDialogue` "RistoCinese" "Non ho visto il gatto." false (`|MakeArray` "" :!type "Text")))
              (switch `/Game/Blueprints/Components/Dialogues/E_DialogueState` _state_6
                (:`NewEnumerator0`
                  (`self.ClearDialogueProgress`)
                  (`self.CloseConversation`))))
            (:`1`
              (`self.ClearDialogueProgress`)
              (`self.CloseConversation`))))))))