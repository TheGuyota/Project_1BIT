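; Dialogue component for Spaccino, the "Shady Guy" NPC who trades a clue about the player's lost cat for help recovering his "sugar".
; A tree index selects the quest offer, turn-in or post-quest chat, built from chained AddDialogue nodes.
; Global parameters gate the offer and an extra monster question.
; Turn-in checks inventory, progresses the objective and swaps the sugar for a bottle, while repeatable branches clear their progress on closing.
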(fn `Dialogue`
  (switch `int` (`self.DialogueTreeIndex`)
    (:`0`
      (bind _state (`self.AddDialogue` "Shady Guy" "OH SHIT! I thought you were a cop! Go away. This is no place for ya, understood?" true (`|MakeArray` "Not now sir, I'm about to find my cat." :!type "Text")))
      (switch `/Game/Blueprints/Components/Dialogues/E_DialogueState` _state
        (:`NewEnumerator0`
          (if (>= (`.Quantity` (`self.QueryGlobalParameters` "Businessman")) 3)
            (bind _state_2 (`self.AddDialogue` "Shady Guy" "Yeah I'm uhhh... I... I need your help. If you help me get my stuff back, I'll tell you something about your cat. Deal?" true (`|MakeArray` "Deal." :!type "Text")))
            (switch `/Game/Blueprints/Components/Dialogues/E_DialogueState` _state_2
              (:`NewEnumerator0`
                (bind _state_3 (`self.AddDialogue` "Shady Guy" "A'ight, some crazy guy tried to rob me and, uh... Nevermind, some of my bags of uhhhh... \"sugar\" flew away in the park." true (`|MakeArray` "I'll help you out!" :!type "Text")))
                (switch `/Game/Blueprints/Components/Dialogues/E_DialogueState` _state_3
                  (:`NewEnumerator0`
                    (`self.SetDialogueTreeIndex` 1)
                    (`self.CloseConversation`))
                  (:`NewEnumerator1`
                    (`self.AddNewQuest` "SpaccinoQuest01")))))
            (else
              (bind _state_4 (`self.AddDialogue` "Shady Guy" "Yeah uhhh... There's no cat here. Now go away, I'm making... affairs. Business affairs, yes." true (`|MakeArray` "At night? In the park...?" :!type "Text")))
              (switch `/Game/Blueprints/Components/Dialogues/E_DialogueState` _state_4
                (:`NewEnumerator0`
                  (bind _state_5 (`self.AddDialogue` "Shady Guy" "Yeah like... trading goods and stuff, y'know." true (`|MakeArray` "May I see em?" :!type "Text")))
                  (switch `/Game/Blueprints/Components/Dialogues/E_DialogueState` _state_5
                    (:`NewEnumerator0`
                      (bind _state_6 (`self.AddDialogue` "Shady Guy" "...No. Get lost!" true (`|MakeArray` "Pfff. meanie!" :!type "Text")))
                      (switch `/Game/Blueprints/Components/Dialogues/E_DialogueState` _state_6
                        (:`NewEnumerator0`
                          (`self.ClearDialogueProgress`)
                          (`self.CloseConversation`))))))))))))
    (:`1`
      (if (== (`/Game/Blueprints/Components/AC_Inventory.QueryInventory` (`/Game/Characters/MainCharacter/BP_MainCharacter.InventoryComponent` (`/Game/Blueprints/CommonFuntionLibrary.GetMyPlayerCharacter`)) "ZuccheroStrano") 1)
        (bind _state_7 (`self.AddDialogue` "Shady Guy" "Soooo uhhh... Found anything?" true (`|MakeArray` "I found this!" :!type "Text")))
        (switch `/Game/Blueprints/Components/Dialogues/E_DialogueState` _state_7
          (:`NewEnumerator0`
            (bind _state_8 (`self.AddDialogue` "Shady Guy" "Geez, thanks little girl! About your cat... I was petting it before the crazy guy threw this bottle to me... But I swear a black cat was here, I even gave it some of my dinner." true (`|MakeArray` "Anything else?" :!type "Text")))
            (switch `/Game/Blueprints/Components/Dialogues/E_DialogueState` _state_8
              (:`NewEnumerator0`
                (bind _state_9 (`self.AddDialogue` "Shady Guy" "Well, maybe just head back home and get some food out! That's how cats work, right?" true (`|MakeArray` "I guess!" :!type "Text")))
                (switch `/Game/Blueprints/Components/Dialogues/E_DialogueState` _state_9
                  (:`NewEnumerator0`
                    (`self.ProgressDialogueQuest` "DaiZuccheroStrano" 1)
                    (`/Game/Blueprints/Components/AC_Inventory.RemoveFromInventory` (`/Game/Characters/MainCharacter/BP_MainCharacter.InventoryComponent` (`/Game/Blueprints/CommonFuntionLibrary.GetMyPlayerCharacter`)) "ZuccheroStrano" 1)
                    (`/Game/Blueprints/Components/AC_Inventory.AddToInventory` (`/Game/Characters/MainCharacter/BP_MainCharacter.InventoryComponent` (`/Game/Blueprints/CommonFuntionLibrary.GetMyPlayerCharacter`)) "Bottiglia" 1)
                    (`self.SetDialogueTreeIndex` 2)
                    (`self.CloseConversation`)))))))
        (else
          (bind _state_10 (`self.AddDialogue` "Shady Guy" "Soooo uhhh... Found anything?" true (`|MakeArray` "Nnnnnnope." :!type "Text")))
          (switch `/Game/Blueprints/Components/Dialogues/E_DialogueState` _state_10
            (:`NewEnumerator0`
              (bind _state_11 (`self.AddDialogue` "Shady Guy" "Shit... My boss is gonna be very angry if I don't have all of them." true (`|MakeArray` "Don't worry about that!" :!type "Text")))
              (switch `/Game/Blueprints/Components/Dialogues/E_DialogueState` _state_11
                (:`NewEnumerator0`
                  (`self.ClearDialogueProgress`)
                  (`self.CloseConversation`))))))))
    (:`2`
      (bind (_state_12 _optionindex) (`self.AddDialogue` "Shady Guy" "OH SHIT! I thought you were a cop! Go away. This is no place for ya, understood?" true (select `bool` (>= (`.Quantity` (`self.QueryGlobalParameters` "Mostro")) 1) :`false` (`|MakeArray` "Why is your sugar so special to you?" :!type "Text") :`true` (`|MakeArray` "Why is your sugar so special to you?" " Are you a monster?" :!type "Text"))))
      (switch `/Game/Blueprints/Components/Dialogues/E_DialogueState` _state_12
        (:`NewEnumerator0`
          (switch `int` _optionindex
            (:`0`
              (bind _state_13 (`self.AddDialogue` "Shady Guy" "Lemme tell ya... It's the worst sugar ever." true (`|MakeArray` "WHAT? Why would people buy it then?" :!type "Text")))
              (switch `/Game/Blueprints/Components/Dialogues/E_DialogueState` _state_13
                (:`NewEnumerator0`
                  (bind _state_14 (`self.AddDialogue` "Shady Guy" "Because... They are too weak to handle normal sugar... I guess. But hey, that's none of your business, okay?" true (`|MakeArray` "You're a weird dude!" :!type "Text")))
                  (switch `/Game/Blueprints/Components/Dialogues/E_DialogueState` _state_14
                    (:`NewEnumerator0`
                      (`self.ClearDialogueProgress`)
                      (`self.CloseConversation`))))))
            (:`1`
              (bind _state_15 (`self.AddDialogue` "Shady Guy" "Me? Uhhh no? Why would you think that?" true (`|MakeArray` "You're hiding in the darkness." :!type "Text")))
              (switch `/Game/Blueprints/Components/Dialogues/E_DialogueState` _state_15
                (:`NewEnumerator0`
                  (bind _state_16 (`self.AddDialogue` "Shady Guy" "I hide in the darkness becauuuuse... Otherwise the monsters would see me! Duh!" true (`|MakeArray` "I'll try hiding, that's a good trick!" :!type "Text")))
                  (switch `/Game/Blueprints/Components/Dialogues/E_DialogueState` _state_16
                    (:`NewEnumerator0`
                      (`self.ClearDialogueProgress`)
                      (`self.CloseConversation`))))))))))))