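; Dialogue component for the Vecchia NPC, who asks the player to find her lost glasses while they search for their cat.
; A switch on DialogueTreeIndex covers the quest offer, glasses check and post-quest brush-off, branching on chosen options.
; Accepting adds VecchiaQuest01, and the turn-in, offered only with Occhiali in the inventory, progresses the DaiOcchiali objective and swaps her sprites.
; Declining paths clear dialogue progress so the conversation can replay.
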(fn `Dialogue`
  (bind _npcselfref (`/Game/Blueprints/CommonFuntionLibrary.GetOwnerNPC` self))
  (switch `int` (`self.DialogueTreeIndex`)
    (:`0`
      (bind (_state _optionindex) (`self.AddDialogue` "Vecchia" "Hey you! I was bringing out the trash and i lost my glasses... Could you find them for me?" true (`|MakeArray` "Alright, I'll find them!" "Sorry, I'm looking for my cat right now." :!type "Text")))
      (switch `/Game/Blueprints/Components/Dialogues/E_DialogueState` _state
        (:`NewEnumerator0`
          (switch `int` _optionindex
            (:`0`
              (bind _state_2 (`self.AddDialogue` "Vecchia" "Heh, thank you! They must be somewhere around the trash cans..." false (`|MakeArray` "" :!type "Text") :!label _label))
              (switch `/Game/Blueprints/Components/Dialogues/E_DialogueState` _state_2
                (:`NewEnumerator0`
                  (`self.SetDialogueTreeIndex` 1)
                  (`self.CloseConversation`))
                (:`NewEnumerator1`
                  (`self.AddNewQuest` "VecchiaQuest01"))))
            (:`1`
              (bind (_state_3 _optionindex_2) (`self.AddDialogue` "Vecchia" "Ahhh, I see. I can tell you something about it, If you help me." true (`|MakeArray` "Pfff... Alright..." "I'm on a hurry, sorry ma'am!" :!type "Text")))
              (switch `/Game/Blueprints/Components/Dialogues/E_DialogueState` _state_3
                (:`NewEnumerator0`
                  (switch `int` _optionindex_2
                    (:`0`
                      (goto _label))
                    (:`1`
                      (bind _state_4 (`self.AddDialogue` "Vecchia" "Ugh... Youngsters nowadays..." false (`|MakeArray` "" :!type "Text")))
                      (switch `/Game/Blueprints/Components/Dialogues/E_DialogueState` _state_4
                        (:`NewEnumerator0`
                          (`self.ClearDialogueProgress`)
                          (`self.CloseConversation`))))))))))))
    (:`1`
      (if (`.bIsFound` (`/Game/Blueprints/Components/AC_Inventory.QueryInventory` (`/Game/Characters/MainCharacter/BP_MainCharacter.InventoryComponent` (`/Game/Blueprints/CommonFuntionLibrary.GetMyPlayerCharacter`)) "Occhiali"))
        (bind (_state_5 _optionindex_3) (`self.AddDialogue` "Vecchia" "So, did you find my glasses?" true (`|MakeArray` "I found 'em. What about my cat? Did you see it?" "Nope, not yet." :!type "Text")))
        (switch `/Game/Blueprints/Components/Dialogues/E_DialogueState` _state_5
          (:`NewEnumerator0`
            (switch `int` _optionindex_3
              (:`0`
                (bind _state_6 (`self.AddDialogue` "Vecchia" "Heh! Thanks! What? Have I seen your cat? I FELL because of your FLEABAG! It was roaming around the rubbish! Now go home, it's late to find your cat anyway!" true (`|MakeArray` "Pff, old fart!" :!type "Text")))
                (switch `/Game/Blueprints/Components/Dialogues/E_DialogueState` _state_6
                  (:`NewEnumerator0`
                    (`self.SetDialogueTreeIndex` 2)
                    (`self.CloseConversation`))
                  (:`NewEnumerator1`
                    (`self.ProgressDialogueQuest` "DaiOcchiali" 1)
                    (`/Game/Blueprints/NPCs/BP_NPC_Master.UpdateDialogueSprite` _npcselfref "/Game/Characters/DialogueCharacters/NPC_Vecchia_B.NPC_Vecchia_B")
                    (`/Game/Blueprints/NPCs/BP_NPC_Master.UpdateWorldSprite` _npcselfref "/Game/Characters/WorldCharacters/Granny/FB_Vecchia_Glasses.FB_Vecchia_Glasses"))))
              (:`1`
                (bind _state_7 (`self.AddDialogue` "Vecchia" "Come on! I can't see anything without them!" false (`|MakeArray` "" :!type "Text") :!label _label_2))
                (switch `/Game/Blueprints/Components/Dialogues/E_DialogueState` _state_7
                  (:`NewEnumerator0`
                    (`self.ClearDialogueProgress`)
                    (`self.CloseConversation`)))))))
        (else
          (bind (_state_8 _optionindex_4) (`self.AddDialogue` "Vecchia" "So, did you find my glasses?" true (`|MakeArray` "Nope, not yet." "I don't remember, where did you lose your glasses?" :!type "Text")))
          (switch `/Game/Blueprints/Components/Dialogues/E_DialogueState` _state_8
            (:`NewEnumerator0`
              (switch `int` _optionindex_4
                (:`0`
                  (goto _label_2))
                (:`1`
                  (bind _state_9 (`self.AddDialogue` "Vecchia" "I lost them around the trash cans near my house... I'm sure they are around here!" false (`|MakeArray` "" :!type "Text")))
                  (switch `/Game/Blueprints/Components/Dialogues/E_DialogueState` _state_9
                    (:`NewEnumerator0`
                      (`self.ClearDialogueProgress`)
                      (`self.CloseConversation`))))))))))
    (:`2`
      (bind _state_10 (`self.AddDialogue` "Vecchia" "You still here? Go home already!" true (`|MakeArray` "Don't tell me what to do!" :!type "Text")))
      (switch `/Game/Blueprints/Components/Dialogues/E_DialogueState` _state_10
        (:`NewEnumerator0`
          (`self.ClearDialogueProgress`)
          (`self.CloseConversation`))))))

(fn `ProgressDialogue`
  (`parent.ProgressDialogue`))