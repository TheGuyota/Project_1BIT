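; Test dialogue component that scripts a branching Italian conversation with the speaker Test1.
; Its Dialogue override calls the parent, then picks one of two trees by DialogueTreeIndex.
; Chained AddDialogue nodes advance on their Pass Through state and branch on the chosen option index.
; Every ending closes the conversation, either clearing dialogue progress or, on one first-tree branch, switching to the second "already talked" tree.
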(fn `Dialogue`
  (`parent.Dialogue`)
  (switch `int` (`self.DialogueTreeIndex`)
    (:`0`
      (bind (_state _optionindex) (`self.AddDialogue` "Test1" "Hey ciao sono un test!" true (`|MakeArray` "Che figo!" "Ma muori!" :!type "Text")))
      (switch `/Game/Blueprints/Components/Dialogues/E_DialogueState` _state
        (:`NewEnumerator0`
          (switch `int` _optionindex
            (:`0`
              (bind _state_2 (`self.AddDialogue` "Test1" "Wow sei un esaltato!" true (`|MakeArray` "Ma.." :!type "Text")))
              (switch `/Game/Blueprints/Components/Dialogues/E_DialogueState` _state_2
                (:`NewEnumerator0`
                  (bind _state_3 (`self.AddDialogue` "Test1" "Dai su, sparisci!" false (`|MakeArray` "" :!type "Text")))
                  (switch `/Game/Blueprints/Components/Dialogues/E_DialogueState` _state_3
                    (:`NewEnumerator0`
                      (`self.ClearDialogueProgress`)
                      (`self.CloseConversation`))))))
            (:`1`
              (bind _state_4 (`self.AddDialogue` "Test1" "Ora mi uccido." false (`|MakeArray` "" :!type "Text")))
              (switch `/Game/Blueprints/Components/Dialogues/E_DialogueState` _state_4
                (:`NewEnumerator0`
                  (`self.SetDialogueTreeIndex` 1)
                  (`self.CloseConversation`))))))))
    (:`1`
      (bind _state_5 (`self.AddDialogue` "Test1" "Abbiamo già parlato, sparisci." false (`|MakeArray` "" :!type "Text")))
      (switch `/Game/Blueprints/Components/Dialogues/E_DialogueState` _state_5
        (:`NewEnumerator0`
          (bind (_state_6 _optionindex_2) (`self.AddDialogue` "Test1" "Aiuuuuto!" true (`|MakeArray` "Uff" "Ci vediamo" :!type "Text")))
          (switch `/Game/Blueprints/Components/Dialogues/E_DialogueState` _state_6
            (:`NewEnumerator0`
              (switch `int` _optionindex_2
                (:`0`
                  (`self.ClearDialogueProgress`)
                  (`self.CloseConversation`))
                (:`1`
                  (bind _state_7 (`self.AddDialogue` "Test1" "E va bene, ciao" false (`|MakeArray` "" :!type "Text")))
                  (switch `/Game/Blueprints/Components/Dialogues/E_DialogueState` _state_7
                    (:`NewEnumerator0`
                      (`self.ClearDialogueProgress`)
                      (`self.CloseConversation`))))))))))))