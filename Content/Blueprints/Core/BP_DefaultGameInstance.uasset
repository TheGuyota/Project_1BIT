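; Game instance that applies startup display settings and resolves the game's ending.
; On Init it caps the frame rate through a console command and remaps PixelDensity into the MCP_DitherPixelDensity parameter collection for dithering.
; The Ending function pauses the game and shows the bad or good ending widget, depending on whether the "Businessman" value in GlobalParameters exceeds a threshold.
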(event `self.ReceiveInit`
  (`KismetSystemLibrary.ExecuteConsoleCommand` "t.MaxFPS 60" (`GameplayStatics.GetPlayerController` 0))
  (`KismetMaterialLibrary.SetScalarParameterValue` "/Game/Shaders/Dither_1Bit/MCP_DitherPixelDensity.MCP_DitherPixelDensity" "PixelDensity" (`KismetMathLibrary.MapRangeClamped` (`self.PixelDensity`) 0.1 1.0 256.0 2048.0)))

(fn `Ending`
  (`GameplayStatics.SetGamePaused` true)
  (if (> (`BlueprintMapLibrary.Map_Find` (`self.GlobalParameters`) "Businessman") 4)
    (bind _returnvalue (`|CreateWidget` "/Game/Widgets/Menu/W_BadEnding.W_BadEnding_C"))
    (`UserWidget.AddToViewport` _returnvalue 0)
    (return)
    (else
      (bind _returnvalue_2 (`|CreateWidget` "/Game/Widgets/Menu/W_GoodEnding.W_GoodEnding_C"))
      (`UserWidget.AddToViewport` _returnvalue_2 0)
      (return))))