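; BP_NPC_Businessman is an NPC Blueprint for a businessman character that relocates in response to game-wide state changes.
; On BeginPlay it subscribes to the global parameter update event on BP_DefaultGameInstance.
; When the updated parameter name matches its CharacterName and the value is 1, it teleports to a fixed world location.
; The construction script only runs the parent's.
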(event `self.ReceiveBeginPlay`
  (bind _asbp_default_game_instance (cast `/Game/Blueprints/Core/BP_DefaultGameInstance` (`GameplayStatics.GetGameInstance`)))
  (add `/Game/Blueprints/Core/BP_DefaultGameInstance.OnGlobalParameterUpdated` _asbp_default_game_instance (delegate `GlobalParameterRelatedEvent`)))

(event `GlobalParameterRelatedEvent`
  (params (Name :type String) (Value :type Integer))
  (if (`KismetStringLibrary.EqualEqual_StrStr` Name (`KismetTextLibrary.Conv_TextToString` (`self.CharacterName`)))
    (switch `int` Value
      (:`1`
        (`self.K2_SetActorLocation` (460.0 -480.0 98.0) false true)))))

(fn `UserConstructionScript`
  (`parent.UserConstructionScript`))