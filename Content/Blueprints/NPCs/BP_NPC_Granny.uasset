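; BP_NPC_Granny is a granny NPC Blueprint that inherits its interaction and construction logic from its parent class, adding nothing to either.
; On BeginPlay it caches the BP_DefaultGameInstance.
; Every Tick it prints each key and value in that instance's GlobalParameters map with zero-duration PrintString, acting as a live debug readout of global state.
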(event `self.ReceiveBeginPlay`
  (bind _asbp_default_game_instance (cast `/Game/Blueprints/Core/BP_DefaultGameInstance` (`GameplayStatics.GetGameInstance`)))
  (set `self.As BP Default Game Instance` _asbp_default_game_instance))

(event `self.ReceiveTick`
  (params (DeltaSeconds :type "Float (single-precision)"))
  (bind _globalparameters (`/Game/Blueprints/Core/BP_DefaultGameInstance.GlobalParameters` (`self.As BP Default Game Instance`)))
  (bind _keys (`BlueprintMapLibrary.Map_Keys` _globalparameters))
  (for _array_element _keys
    (`KismetSystemLibrary.PrintString` (`KismetStringLibrary.Concat_StrStr` _array_element ": " (`KismetStringLibrary.Conv_IntToString` (`BlueprintMapLibrary.Map_Find` _globalparameters _array_element))) true true (struct :`G` 0.66 :`B` 1.0 :`A` 1.0) 0.0)))

(fn `Interact`
  (params (Instigator :type "Actor Object Reference"))
  (returns (ObjectiveID :type String))
  (bind _objectiveid (`parent.Interact` Instigator))
  (return _objectiveid))

(fn `UserConstructionScript`
  (`parent.UserConstructionScript`))