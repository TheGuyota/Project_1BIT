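; BP_NPC_Master is an interactable NPC with a flipbook sprite, dialogue and quest giving.
; Interact starts the conversation on its AC_Dialogue_Master component, if present, then calls the QuestGiverComponent.
; Update functions change location, name, sprites and quest data, and can swap dialogue components by class at runtime.
; A dialogue cloud shows interactability, and GiveQuestDialogue adds quests not already active to the player's quest log.
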(event `/Game/Blueprints/Interfaces/BPI_Interaction.SetInteractableState`
  (params (bCanShowInteraction :type Boolean))
  (bind _dialoguecloud (`self.DialogueCloud`))
  (if bCanShowInteraction
    (`SceneComponent.SetVisibility` _dialoguecloud true false)
    (else
      (`SceneComponent.SetVisibility` _dialoguecloud false false))))

(fn `ConversationClosed`
  (return))

(fn `GiveQuest_Dialogue`
  (params (QuestID :type Name))
  (if (not (`/Game/Blueprints/QuestSystem/AC_QuestLog.QueryActiveQuest` (`/Game/Characters/MainCharacter/BP_MainCharacter.QuestLogComponent` (`/Game/Blueprints/CommonFuntionLibrary.GetMyPlayerCharacter`)) QuestID))
    (`/Game/Blueprints/QuestSystem/AC_QuestLog.AddNewQuest` (`/Game/Characters/MainCharacter/BP_MainCharacter.QuestLogComponent` (`/Game/Blueprints/CommonFuntionLibrary.GetMyPlayerCharacter`)) (`local.QuestID`))))

(fn `Interact`
  (params (Instigator :type "Actor Object Reference"))
  (returns (ObjectiveID :type String))
  (bind _returnvalue (`self.GetComponentByClass` "/Game/Blueprints/Components/Dialogues/AC_Dialogue_Master.AC_Dialogue_Master_C"))
  (set `self.InteractionInstigator` Instigator)
  (`/Engine/EditorBlueprintResources/StandardMacros.IsValid` _returnvalue
    (:`Is Valid`
      (`/Game/Blueprints/Components/Dialogues/AC_Dialogue_Master.StartConversation` _returnvalue))
    (:`Is Not Valid`
      _))
  (`/Game/Blueprints/QuestSystem/AC_QuestGiver.Interact` (`self.QuestGiverComponent`) (`/Game/Blueprints/CommonFuntionLibrary.GetMyPlayerCharacter`))
  (return (`KismetTextLibrary.Conv_TextToString` (`self.CharacterName`))))

(fn `UpdateCharacterName`
  (params (CharacterName :type Text))
  (set `self.CharacterName` CharacterName)
  (return))

(fn `UpdateDialogueSprite`
  (params (DialogueSprite :type "Texture2D Object Reference"))
  (set `/Game/Blueprints/Components/Dialogues/AC_Dialogue_Master.RightSpeaker` DialogueSprite (`self.GetComponentByClass` "/Game/Blueprints/Components/Dialogues/AC_Dialogue_Master.AC_Dialogue_Master_C"))
  (return))

(fn `UpdateDialogueSystem`
  (params (DialogueComponentToRemove :type "/Game/Blueprints/Components/Dialogues/AC_Dialogue_Master Object Reference") (DIalogueComponentToAdd :type "/Game/Blueprints/Components/Dialogues/AC_Dialogue_Master Class Reference"))
  (`ActorComponent.K2_DestroyComponent` DialogueComponentToRemove)
  (if (`KismetSystemLibrary.IsValidClass` DIalogueComponentToAdd)
    (`|AddComponentByClass` DIalogueComponentToAdd null null null)
    (return)
    (else
      (return))))

(fn `UpdateQuest`
  (params (QuestData :type "DataTableRowHandle Structure"))
  (returns (ObjectiveID :type String))
  (set `/Game/Blueprints/QuestSystem/AC_QuestGiver.QuestData` QuestData (`self.QuestGiverComponent`))
  (return (`KismetTextLibrary.Conv_TextToString` (`self.CharacterName`))))

(fn `UpdateSelfLocation`
  (params (NewLocation :type "Vector Structure"))
  (`self.K2_SetActorLocation` NewLocation false true)
  (return))

(fn `UpdateWorldSprite`
  (params (WorldSprite :type "PaperFlipbook Object Reference"))
  (`PaperFlipbookComponent.SetFlipbook` (`self.Sprite`) WorldSprite)
  (return))

(fn `UserConstructionScript`)