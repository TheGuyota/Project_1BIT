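; BP_Pickupable_Collare is a pickupable collar that the player collects by interacting with it.
; Interact adds the item to the player's inventory, calls the "Ending" objective if "Ciotola" and "Latte" are also held, and refreshes the inventory container.
; It then increments the "Businessman" global parameter in the game instance, broadcasts the update, destroys itself and returns the item name.
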(fn `Interact`
  (params (Instigator :type "Actor Object Reference"))
  (returns (ObjectiveID :type String))
  (bind _maincharacter (`/Game/Blueprints/CommonFuntionLibrary.GetMyPlayerCharacter`))
  (set `self.InteractionInstigator` Instigator)
  (`/Game/Blueprints/Components/AC_Inventory.AddToInventory` (`/Game/Characters/MainCharacter/BP_MainCharacter.InventoryComponent` _maincharacter) (`self.ItemName`) (`self.Quantity`))
  (if (and (`.bIsFound` (`/Game/Blueprints/Components/AC_Inventory.QueryInventory` (`/Game/Characters/MainCharacter/BP_MainCharacter.InventoryComponent` (`/Game/Blueprints/CommonFuntionLibrary.GetMyPlayerCharacter`)) "Ciotola")) (`.bIsFound` (`/Game/Blueprints/Components/AC_Inventory.QueryInventory` (`/Game/Characters/MainCharacter/BP_MainCharacter.InventoryComponent` (`/Game/Blueprints/CommonFuntionLibrary.GetMyPlayerCharacter`)) "Latte")))
    (`/Game/Characters/MainCharacter/BP_MainCharacter.OnObjectiveIDCalled` (`/Game/Blueprints/CommonFuntionLibrary.GetMyPlayerCharacter`) "Ending" 1))
  (`/Game/Characters/MainCharacter/BP_MainCharacter.UpdateInventoryContainer` _maincharacter)
  (bind _asbp_default_game_instance (cast `/Game/Blueprints/Core/BP_DefaultGameInstance` (`GameplayStatics.GetGameInstance`)))
  (bind _globalparameters (`/Game/Blueprints/Core/BP_DefaultGameInstance.GlobalParameters` _asbp_default_game_instance))
  (`BlueprintMapLibrary.Map_Add` _globalparameters "Businessman" (+ (`BlueprintMapLibrary.Map_Find` (`/Game/Blueprints/Core/BP_DefaultGameInstance.GlobalParameters` _asbp_default_game_instance) "Businessman") 1))
  (`/Game/Blueprints/Core/BP_DefaultGameInstance.OnGlobalParameterUpdated` _asbp_default_game_instance "Businessman" (`BlueprintMapLibrary.Map_Find` _globalparameters "Businessman"))
  (`self.K2_DestroyActor`)
  (return (`KismetStringLibrary.Conv_NameToString` (`self.ItemName`))))

(fn `UserConstructionScript`
  (`parent.UserConstructionScript`))