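; Base pickupable actor that adds its item and quantity to the player's inventory on interaction, then destroys itself.
; When the player's capsule overlaps its Box, it shows an Indicator and starts a bobbing loop, hiding and stopping it on exit.
; The bob alternates a Z timeline forward and backward through a FlipFlop, re-triggered when the timeline finishes.
; Interact also refreshes the inventory container and returns the item name.
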(event `DanceLoop`
  (bind _indicator (`self.Indicator`))
  (bind (_relativelocation_x _relativelocation_y) (`KismetMathLibrary.BreakVector` (`SceneComponent.RelativeLocation` _indicator)))
  (if (`self.bCanDanceLoop`)
    (`/Engine/EditorBlueprintResources/StandardMacros.FlipFlop`
      (:`A`
        (bind (_direction _zvalue) (`Timeline|ZValue` :!label _label)
          (:`Update`
            (`SceneComponent.K2_SetRelativeLocation` _indicator (`KismetMathLibrary.MakeVector` _relativelocation_x _relativelocation_y (`KismetMathLibrary.MapRangeClamped` _zvalue 0.0 1.0 30.0 70.0)) false false))
          (:`Finished`
            (`self.DanceLoop`))))
      (:`B`
        (goto _label :!via `Reverse`)))))

(event `self.Box.OnComponentBeginOverlap`
  (params (OverlappedComponent :type "PrimitiveComponent Object Reference") (OtherActor :type "Actor Object Reference") (OtherComp :type "PrimitiveComponent Object Reference") (OtherBodyIndex :type Integer) (bFromSweep :type Boolean) (SweepResult :type "HitResult Structure (by ref)"))
  (if (`self.ActorHasTag` OtherActor "Player")
    (cast `CapsuleComponent` OtherComp)
    (set `self.bCanDanceLoop` true)
    (`self.DanceLoop`)
    (`SceneComponent.SetHiddenInGame` (`self.Indicator`) false false)))

(event `self.Box.OnComponentEndOverlap`
  (params (OverlappedComponent :type "PrimitiveComponent Object Reference") (OtherActor :type "Actor Object Reference") (OtherComp :type "PrimitiveComponent Object Reference") (OtherBodyIndex :type Integer))
  (if (`self.ActorHasTag` OtherActor "Player")
    (cast `CapsuleComponent` OtherComp)
    (set `self.bCanDanceLoop` false)
    (`SceneComponent.SetHiddenInGame` (`self.Indicator`) true false)))

(fn `Interact`
  (params (Instigator :type "Actor Object Reference"))
  (returns (ObjectiveID :type String))
  (bind _maincharacter (`/Game/Blueprints/CommonFuntionLibrary.GetMyPlayerCharacter`))
  (set `self.InteractionInstigator` Instigator)
  (`/Game/Blueprints/Components/AC_Inventory.AddToInventory` (`/Game/Characters/MainCharacter/BP_MainCharacter.InventoryComponent` _maincharacter) (`self.ItemName`) (`self.Quantity`))
  (`/Game/Characters/MainCharacter/BP_MainCharacter.UpdateInventoryContainer` _maincharacter)
  (`self.K2_DestroyActor`)
  (return (`KismetStringLibrary.Conv_NameToString` (`self.ItemName`))))

(fn `UserConstructionScript`)