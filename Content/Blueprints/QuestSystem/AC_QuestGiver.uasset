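; Actor component that makes its owner a quest giver for the quest named by its QuestData row.
; Interact checks the player's QuestLogComponent and, if the quest is neither active nor completed, calls DisplayQuest, which adds it to the log directly.
; Otherwise, it collects rewards when the quest actor is completed but not yet redeemed.
; Both successful paths return the owner's display name, and the ConversationClosed event is empty.
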(event `/Game/Blueprints/Interfaces/BPI_Interaction.ConversationClosed`)

(fn `DisplayQuest`
  (bind (_questdata_datatable _questdata_rowname) (break `DataTableRowHandle` (`self.QuestData`)))
  (bind _questlogcomponent (`/Game/Characters/MainCharacter/BP_MainCharacter.QuestLogComponent` (`/Game/Blueprints/CommonFuntionLibrary.GetMyPlayerCharacter`))
    (:`then`
      (`/Game/Blueprints/QuestSystem/AC_QuestLog.AddNewQuest` _questlogcomponent _questdata_rowname))
    (:`else`)))

(fn `Interact`
  (params (Instigator :type "Actor Object Reference"))
  (returns (ObjectiveID :type String))
  (bind (_questdata_datatable _questdata_rowname) (break `DataTableRowHandle` (`self.QuestData`)))
  (bind _returnvalue (`KismetSystemLibrary.GetDisplayName` (`self.GetOwner`)))
  (bind _questlogcomponent (`/Game/Characters/MainCharacter/BP_MainCharacter.QuestLogComponent` (`/Game/Blueprints/CommonFuntionLibrary.GetMyPlayerCharacter`)))
  (bind _questlogcomponent_2 (`/Game/Characters/MainCharacter/BP_MainCharacter.QuestLogComponent` (`/Game/Blueprints/CommonFuntionLibrary.GetMyPlayerCharacter`)))
  (bind _questactor (`/Game/Blueprints/QuestSystem/AC_QuestLog.GetQuestActor` _questlogcomponent _questdata_rowname))
  (if (and (not (`/Game/Blueprints/QuestSystem/AC_QuestLog.QueryActiveQuest` _questlogcomponent_2 _questdata_rowname)) (not (`/Game/Blueprints/QuestSystem/AC_QuestLog.QueryCompletedQuest` _questlogcomponent_2 _questdata_rowname)))
    (`self.DisplayQuest`)
    (return _returnvalue)
    (elif (and (`/Game/Blueprints/QuestSystem/BP_QuestSystem_Base.bIsCompleted` _questactor) (not (`/Game/Blueprints/QuestSystem/BP_QuestSystem_Base.bIsRedeemed` _questactor)))
      (`/Game/Blueprints/QuestSystem/AC_QuestLog.CollectQuestRewards` _questlogcomponent _questdata_rowname)
      (return _returnvalue))))