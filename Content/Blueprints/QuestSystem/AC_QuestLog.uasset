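; Quest log component that tracks the player's active and completed quests by ID.
; Adding a quest spawns a BP_QuestSystem_Base actor to represent it and passes it to the in-game UI tracker.
; Collecting rewards puts the current stage's items into the player's inventory, then completes the quest, marking it redeemed and broadcasting OnQuestCompleted.
; Query functions report quest status, treating quests without an actor as redeemed; TrackQuest is an empty stub.
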(fn `AddNewQuest`
  (params (QuestID :type Name))
  (`KismetArrayLibrary.Array_AddUnique` (`self.CurrentActiveQuests`) QuestID)
  (bind _returnvalue (`|SpawnActorFromClass` "/Game/Blueprints/QuestSystem/BP_QuestSystem_Base.BP_QuestSystem_Base_C" (`KismetMathLibrary.MakeTransform` (0.0 0.0 0.0)) "Undefined" "MultiplyWithRoot" null QuestID null))
  (`KismetArrayLibrary.Array_Add` (`self.CurrentQuests`) _returnvalue)
  (`/Game/Widgets/W_InGameUI.UpdateQuestTracker` (`/Game/Characters/MainCharacter/BP_MainCharacter.InGameUI` (`/Game/Blueprints/CommonFuntionLibrary.GetMyPlayerCharacter`)) _returnvalue))

(fn `CollectQuestRewards`
  (params (QuestID :type Name))
  (bind ((`ItemRewards_14_8B7F9E81424C630E71794BBB407D03D5` _itemrewards)) (break `/Game/Blueprints/QuestSystem/S_StageDetails` (`/Game/Blueprints/QuestSystem/BP_QuestSystem_Base.CurrentStageDetails` (`self.GetQuestActor` (`local.QuestID`)))))
  (`|ExecutionSequence`
    (:`then_0`
      (bind _keys (`BlueprintMapLibrary.Map_Keys` _itemrewards))
      (for _array_element _keys
        (`/Game/Blueprints/Components/AC_Inventory.AddToInventory` (`/Game/Characters/MainCharacter/BP_MainCharacter.InventoryComponent` (`/Game/Blueprints/CommonFuntionLibrary.GetMyPlayerCharacter`)) _array_element (`BlueprintMapLibrary.Map_Find` _itemrewards _array_element))))
    (:`then_1`
      (`self.CompleteQuest` QuestID))))

(fn `CompleteQuest`
  (params (QuestID :type Name))
  (bind _questactor (`self.GetQuestActor` QuestID))
  (`KismetArrayLibrary.Array_Add` (`self.CompletedQuests`) QuestID)
  (`KismetArrayLibrary.Array_RemoveItem` (`self.CurrentActiveQuests`) QuestID)
  (set `/Game/Blueprints/QuestSystem/BP_QuestSystem_Base.bIsRedeemed` true _questactor)
  (`self.OnQuestCompleted` _questactor)
  (return))

(fn `GetQuestActor`
  (params (QuestID :type Name))
  (returns (QuestActor :type "/Game/Blueprints/QuestSystem/BP_QuestSystem_Base Object Reference"))
  (for _array_element (`self.CurrentQuests`)
    (if (== (`/Game/Blueprints/QuestSystem/BP_QuestSystem_Base.QuestID` _array_element) (`local.QuestID`))
      (return _array_element))))

(fn `QueryActiveQuest`
  (params (QuestID :type Name))
  (returns (ReturnValue :type Boolean))
  (return (`KismetArrayLibrary.Array_Contains` (`self.CurrentActiveQuests`) QuestID)))

(fn `QueryCompletedQuest`
  (params (QuestID :type Name))
  (returns (ReturnValue :type Boolean) (bIsRedeemed :type Boolean))
  (bind _questactor (`self.GetQuestActor` QuestID))
  (bind _returnvalue (`KismetArrayLibrary.Array_Contains` (`self.CompletedQuests`) QuestID))
  (`/Engine/EditorBlueprintResources/StandardMacros.IsValid` _questactor
    (:`Is Valid`
      (return _returnvalue (`/Game/Blueprints/QuestSystem/BP_QuestSystem_Base.bIsRedeemed` _questactor)))
    (:`Is Not Valid`
      (return _returnvalue true))))

(fn `TrackQuest`)