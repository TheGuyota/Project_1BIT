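; Base quest tracker that loads a quest's stages from DT_QuestData and tracks objective progress for the current stage.
; It listens to the player's objective-ID event, and at BeginPlay feeds inventory counts into objectives of one type.
; Completed objectives show a notification widget; once all are met, the next stage loads.
; After the last stage the quest is marked completed, and auto-complete quests collect rewards through the player's QuestLogComponent.
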(event `self.ReceiveBeginPlay`
  (`self.GetQuestDetails`)
  (add `/Game/Characters/MainCharacter/BP_MainCharacter.OnObjectiveIDCalled` (`/Game/Blueprints/CommonFuntionLibrary.GetMyPlayerCharacter`) (`|CreateDelegate` :!event `OnObjectiveIDHeard`))
  (for _array_element (`.Objective_17_9DD66D554C95083ABA26ACB0BBF8D4D7` (break `/Game/Blueprints/QuestSystem/S_StageDetails` (`self.CurrentStageDetails`)))
    (bind ((`Type_17_8F1A58E840291413A24B348EF0D74963` _type) (`ObjectiveID_9_347DD7A441E42E91830239B88931ADF5` _objectiveid)) (break `/Game/Blueprints/QuestSystem/S_ObjectiveDetails` _array_element))
    (if (`|EnumEquality` _type "NewEnumerator3")
      (`self.OnObjectiveIDHeard` _objectiveid (`/Game/Blueprints/Components/AC_Inventory.QueryInventory` (`/Game/Characters/MainCharacter/BP_MainCharacter.InventoryComponent` (`/Game/Blueprints/CommonFuntionLibrary.GetMyPlayerCharacter`)) (`KismetStringLibrary.Conv_StringToName` _objectiveid))))))

(fn `Are All Objective Complete`
  (returns (ReturnValue :type Boolean))
  (locals (Local_AllComplete :type Boolean :default true))
  (for _array_element (`.Objective_17_9DD66D554C95083ABA26ACB0BBF8D4D7` (break `/Game/Blueprints/QuestSystem/S_StageDetails` (`self.CurrentStageDetails`)))
    (bind (_objectivename _description _type _objectiveid) (break `/Game/Blueprints/QuestSystem/S_ObjectiveDetails` _array_element))
    (if (not (>= (`BlueprintMapLibrary.Map_Find` (`self.CurrentObjectiveProgress`) _objectiveid) (`.Quantity_12_F5DB2E5547D8A33DA200F6A6AA47CAAA` (break `/Game/Blueprints/QuestSystem/S_ObjectiveDetails` (`self.GetObjectiveDataByID` _objectiveid)))))
      (bind _output_get (set `local.Local_AllComplete` false))
      (return _output_get)))
  (return (`local.Local_AllComplete`)))

(fn `GetObjectiveDataByID`
  (params (ObjectiveID :type String))
  (returns (ObjectiveDetails :type "/Game/Blueprints/QuestSystem/S_ObjectiveDetails Structure"))
  (for _array_element (`.Objective_17_9DD66D554C95083ABA26ACB0BBF8D4D7` (break `/Game/Blueprints/QuestSystem/S_StageDetails` (`self.CurrentStageDetails`)))
    (if (`KismetStringLibrary.EqualEqual_StrStr` (`.ObjectiveID_9_347DD7A441E42E91830239B88931ADF5` (break `/Game/Blueprints/QuestSystem/S_ObjectiveDetails` _array_element)) (`local.ObjectiveID`))
      (return _array_element))))

(fn `GetQuestDetails`
  (bind (_currentstagedetails_stagename _currentstagedetails_description _currentstagedetails_objective) (break `/Game/Blueprints/QuestSystem/S_StageDetails` (`self.CurrentStageDetails`)))
  (bind _returnvalue (`|GetDataTableRow` "/Game/Blueprints/QuestSystem/DT_QuestData.DT_QuestData" (`self.QuestID`))
    (:`then`
      (bind _output_get (set `self.QuestDetails` _returnvalue))
      (set `self.CurrentStageDetails` (`|GetArrayItem` (`.Stages_16_0BBD8D5143C6A3E053EE3DB4AD94070D` (break `/Game/Blueprints/QuestSystem/S_QuestDetails` _output_get)) (`self.CurrentStage`)))
      (`BlueprintMapLibrary.Map_Clear` (`self.CurrentObjectiveProgress`))
      (for _array_element _currentstagedetails_objective
        (`BlueprintMapLibrary.Map_Add` (`self.CurrentObjectiveProgress`) (`.ObjectiveID_9_347DD7A441E42E91830239B88931ADF5` (break `/Game/Blueprints/QuestSystem/S_ObjectiveDetails` _array_element)))))))

(fn `IsObjectiveComplete`
  (params (ObjectiveID :type String))
  (bind (_questdetails_questname _questdetails_logdescription _questdetails_trackingdescription _questdetails_bismainquest _questdetails_stages _questdetails_bautocomplete) (break `/Game/Blueprints/QuestSystem/S_QuestDetails` (`self.QuestDetails`)))
  (bind ((`ObjectiveName_2_79132B0B4BBE4911598B48B1F731E074` _objectivename) (`Quantity_12_F5DB2E5547D8A33DA200F6A6AA47CAAA` _quantity)) (break `/Game/Blueprints/QuestSystem/S_ObjectiveDetails` (`self.GetObjectiveDataByID` ObjectiveID)))
  (if (>= (`BlueprintMapLibrary.Map_Find` (`self.CurrentObjectiveProgress`) (`local.ObjectiveID`)) _quantity)
    (bind _returnvalue (`|CreateWidget` "/Game/Widgets/QuestSystem/W_QuestNotification.W_QuestNotification_C" null _objectivename))
    (`UserWidget.AddToViewport` _returnvalue 0)
    (bind _returnvalue_2 (`self.Are All Objective Complete`))
    (if _returnvalue_2
      (bind _result (`/Engine/EditorBlueprintResources/StandardMacros.IncrementInt` (`self.CurrentStage`))
        (:`  `
          (if (`KismetArrayLibrary.Array_IsValidIndex` (`.Stages_16_0BBD8D5143C6A3E053EE3DB4AD94070D` (break `/Game/Blueprints/QuestSystem/S_QuestDetails` (`self.QuestDetails`))) _result)
            (`self.GetQuestDetails`)
            (else
              (set `self.bIsCompleted` true)
              (if _questdetails_bautocomplete
                (`/Game/Blueprints/QuestSystem/AC_QuestLog.CollectQuestRewards` (`/Game/Characters/MainCharacter/BP_MainCharacter.QuestLogComponent` (`/Game/Blueprints/CommonFuntionLibrary.GetMyPlayerCharacter`)) (`self.QuestID`))))))))))

(fn `OnObjectiveIDHeard`
  (params (ObjectiveID :type String) (Value :type Integer :default 1))
  (bind (_value _returnvalue) (`BlueprintMapLibrary.Map_Find` (`self.CurrentObjectiveProgress`) (`local.ObjectiveID`)))
  (if (> (`KismetMathLibrary.SignOfInteger` Value) 0)
    (if _returnvalue
      (if (< _value (`.Quantity_12_F5DB2E5547D8A33DA200F6A6AA47CAAA` (break `/Game/Blueprints/QuestSystem/S_ObjectiveDetails` (`self.GetObjectiveDataByID` (`local.ObjectiveID`)))))
        (`BlueprintMapLibrary.Map_Add` (`self.CurrentObjectiveProgress`) (`local.ObjectiveID`) (+ _value (`local.Value`)))
        (`self.IsObjectiveComplete` (`local.ObjectiveID`))
        (`self.OnObjectiveHeard`)
        (return))
      (else
        (return)))
    (else
      (`BlueprintMapLibrary.Map_Add` (`self.CurrentObjectiveProgress`) (`local.ObjectiveID`) (+ (`BlueprintMapLibrary.Map_Find` (`self.CurrentObjectiveProgress`) (`local.ObjectiveID`)) (`local.Value`)))
      (return))))

(fn `UserConstructionScript`)