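; Monster enemy that chases the player with AI Move To, whispering and bobbing its flipbook sprite, and triggers game over when its kill range touches the player.
; BeginPlay randomizes speed, float range and light resistance; a flip-flopped Timeline drives the bob.
; Start/StopLighting use paired DoOnce gates to run or cancel a resistance timer.
; When it expires, the monster increments the GameInstance "Mostro" count, stops, swaps sprite and despawns.
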(event `StopDanceLoop`
  (bind _sprite (`self.Sprite`))
  (bind (_relativelocation_x _relativelocation_y) (`KismetMathLibrary.BreakVector` (`SceneComponent.RelativeLocation` _sprite)))
  (set `self.bCanDanceLoop` false)
  (bind (_direction _zvalue) (`Timeline|Timeline` :!via `Stop` :!label _label)
    (:`Update`
      (`SceneComponent.K2_SetRelativeLocation` _sprite (`KismetMathLibrary.MakeVector` _relativelocation_x _relativelocation_y (`KismetMathLibrary.MapRangeClamped` _zvalue 0.0 1.0 (`self.FloatingMin`) (`self.FloatingMax`))) false false))
    (:`Finished`
      (`self.DanceLoop`))))

(event `DanceLoop`
  (if (`self.bCanDanceLoop`)
    (`/Engine/EditorBlueprintResources/StandardMacros.FlipFlop`
      (:`A`
        (goto _label))
      (:`B`
        (goto _label :!via `Reverse`)))))

(event `self.ReceiveTick`
  (params (DeltaSeconds :type "Float (single-precision)"))
  (`KismetSystemLibrary.PrintString` (`KismetSystemLibrary.GetDisplayName` self) true true (struct :`G` 0.66 :`B` 1.0 :`A` 1.0) 0.0))

(event `self.ReceiveBeginPlay`
  (set `CharacterMovementComponent.MaxWalkSpeed` (`KismetMathLibrary.RandomFloatInRange` 200.0 350.0) (`self.CharacterMovement`))
  (set `self.FloatingMin` (`KismetMathLibrary.RandomFloatInRange` -10.0 20.0))
  (set `self.FloatingMax` (`KismetMathLibrary.RandomFloatInRange` 50.0 90.0))
  (set `self.Resistance` (`KismetMathLibrary.RandomFloatInRange` 0.25 1.5))
  (bind _returnvalue (`GameplayStatics.SpawnSoundAttached` (`KismetArrayLibrary.Array_Random` (`|MakeArray` "/Game/SFX/Sounds/Whisper_1_Cue.Whisper_1_Cue" "/Game/SFX/Sounds/Whisper_2_Cue.Whisper_2_Cue" :!type "SoundBase Object Reference")) (`self.Sprite`) "None" (0.0 0.0 0.0) (struct) "KeepRelativeOffset" false 0.5 1.0 0.0 "/Game/SFX/SA_Whisper.SA_Whisper" null false))
  (set `self.WhisperSound` _returnvalue)
  (`|AIMoveTo` self (0.0 0.0 0.0) (`GameplayStatics.GetPlayerCharacter` 0)
    (:`then`
      (`self.DanceLoop`))))

(event `/Game/Blueprints/Interfaces/BPI_Monster.StartLighting`
  (`/Engine/EditorBlueprintResources/StandardMacros.DoOnce` false :!label _label_2
    (:`Completed`
      (bind _returnvalue (`KismetSystemLibrary.K2_SetTimerDelegate` (delegate `Lighting`) (`self.Resistance`)))
      (set `self.LightingHandle` _returnvalue)
      (bind _returnvalue_2 (`KismetSystemLibrary.K2_SetTimerDelegate` (delegate `Countdown`) 0.01 true))
      (set `self.CountdownHandle` _returnvalue_2)
      (goto _label_3 :!via `Reset`))))

(event `/Game/Blueprints/Interfaces/BPI_Monster.StopLighting`
  (`/Engine/EditorBlueprintResources/StandardMacros.DoOnce` false :!label _label_3
    (:`Completed`
      (set `self.Counter` 0.0)
      (`KismetSystemLibrary.K2_ClearAndInvalidateTimerHandle` (`self.CountdownHandle`))
      (`KismetSystemLibrary.K2_ClearAndInvalidateTimerHandle` (`self.LightingHandle`))
      (goto _label_2 :!via `Reset`))))

(event `Lighting`
  (`self.DeathActions`))

(event `Countdown`
  (set `self.Counter` (+ (`self.Counter`) 0.01)))

(event `self.KillRange.OnComponentBeginOverlap`
  (params (OverlappedComponent :type "PrimitiveComponent Object Reference") (OtherActor :type "Actor Object Reference") (OtherComp :type "PrimitiveComponent Object Reference") (OtherBodyIndex :type Integer) (bFromSweep :type Boolean) (SweepResult :type "HitResult Structure (by ref)"))
  (if (`self.ActorHasTag` OtherActor "Player")
    (`/Game/Characters/MainCharacter/BP_MainCharacter.GameOver` (`/Game/Blueprints/CommonFuntionLibrary.GetMyPlayerCharacter`))))

(fn `DeathActions`
  (`/Engine/EditorBlueprintResources/StandardMacros.DoOnce` false
    (:`Completed`
      (bind _asbp_default_game_instance (cast `/Game/Blueprints/Core/BP_DefaultGameInstance` (`GameplayStatics.GetGameInstance`))
        (:`then`
          (bind _globalparameters (`/Game/Blueprints/Core/BP_DefaultGameInstance.GlobalParameters` _asbp_default_game_instance))
          (`BlueprintMapLibrary.Map_Add` _globalparameters "Mostro" (+ (`BlueprintMapLibrary.Map_Find` _globalparameters "Mostro") 1)))
        (:`CastFailed`
          _))
      (`PrimitiveComponent.SetCollisionEnabled` (`self.KillRange`) "NoCollision")
      (`MovementComponent.StopMovementImmediately` (`self.CharacterMovement`))
      (`PaperFlipbookComponent.SetFlipbook` (`self.Sprite`) (`KismetArrayLibrary.Array_Random` (`|MakeArray` "/Game/Characters/Monster/Enemy_cioccato_Flipbook.Enemy_cioccato_Flipbook" "/Game/Characters/Monster/Enemy_cioccato1.Enemy_cioccato1" :!type "PaperFlipbook Object Reference")))
      (`self.StopDanceLoop`)
      (`AudioComponent.Stop` (`self.WhisperSound`))
      (`GameplayStatics.PlaySoundAtLocation` "/Game/SFX/Sounds/Monster_Mumble_Cue.Monster_Mumble_Cue" (`self.K2_GetActorLocation`) (struct) 1.0 1.0 0.0 null null null null)
      (`self.SetLifeSpan` 2.0))))

(fn `UserConstructionScript`)